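; Enemy grenade character that hurls itself toward the player when it spawns.
; On BeginPlay it applies a velocity-change impulse to its capsule, aimed at the player's XY position at world Z zero and scaled by Speed, so strength grows with distance.
; Unconnected leftover nodes hold a LaunchCharacter alternative and a projectile path prediction with a debug landing trace.
; The graph contains no detonation or damage logic.
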(event `self.ReceiveBeginPlay`
  (bind (_returnvalue_x _returnvalue_y) (`KismetMathLibrary.BreakVector` (`self.K2_GetActorLocation` (`GameplayStatics.GetPlayerCharacter` 0))))
  (`PrimitiveComponent.AddImpulse` (`self.CapsuleComponent`) (* (- (`KismetMathLibrary.MakeVector` _returnvalue_x _returnvalue_y) (`self.K2_GetActorLocation`)) (`self.Speed`)) "None" true))

(fn `UserConstructionScript`)