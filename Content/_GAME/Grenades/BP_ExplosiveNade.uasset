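; BP_ExplosiveNade is a thrown explosive grenade that detonates on a timed fuse.
; Throw unhides its widget and launches the mesh with a velocity-change impulse along the GetInstance actor's forward vector, plus a fraction of that actor's velocity.
; After a short delay it spawns an explosion emitter, fires a RadialForce impulse, plays the explosion sound and destroys itself.
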(event `self.Throw`
  (`SceneComponent.SetHiddenInGame` (`self.Widget`) false false)
  (bind _returnvalue (`MyCharacter.GetInstance`))
  (`PrimitiveComponent.AddImpulse` (`self.Mesh`) (+ (* (`self.GetActorForwardVector` _returnvalue) 500.0) (/ (`self.GetVelocity` _returnvalue) 20.0)) "None" true)
  (`KismetSystemLibrary.Delay` 2.0)
  (`GameplayStatics.SpawnEmitterAtLocation` "/Game/MilitaryWeapSilver/FX/P_Grenade_Explosion_01.P_Grenade_Explosion_01" (`self.K2_GetActorLocation`))
  (`RadialForceComponent.FireImpulse` (`self.RadialForce`))
  (`GameplayStatics.PlaySoundAtLocation` "/Game/MilitaryWeapSilver/Sound/GrenadeLauncher/Cues/GrenadeLauncher_Explosion_Cue.GrenadeLauncher_Explosion_Cue" (`self.K2_GetActorLocation`) (struct) 1.0 1.0 0.0 null null null)
  (`self.K2_DestroyActor`))

(fn `UserConstructionScript`
  (`parent.UserConstructionScript`))