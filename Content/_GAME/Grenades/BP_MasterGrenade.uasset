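; Master grenade actor that launches itself from the player, then explodes after a short fixed fuse.
; On BeginPlay it applies a velocity-change impulse to its mesh, combining the main player character's forward vector with half that character's velocity.
; When the delay ends it spawns an explosion particle, fires its RadialForce impulse to push nearby objects and destroys itself, with no explicit damage call.
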(event `self.ReceiveBeginPlay`
  (bind (_asmaingamemode _asmainplayercontroller _asmainplayercharacter) (`BPFunctionLibrary.CastToCore_Main` self))
  (set `self.As Main Player Character` _asmainplayercharacter)
  (`PrimitiveComponent.AddImpulse` (`self.Mesh`) (+ (* (`self.GetActorForwardVector` (`self.As Main Player Character`)) 500.0) (/ (`self.GetVelocity` (`self.As Main Player Character`)) 2.0)) "None" true)
  (`KismetSystemLibrary.Delay` 2.0)
  (`GameplayStatics.SpawnEmitterAtLocation` "/Game/MilitaryWeapSilver/FX/P_Grenade_Explosion_01.P_Grenade_Explosion_01" (`self.K2_GetActorLocation`))
  (`RadialForceComponent.FireImpulse` (`self.RadialForce`))
  (`self.K2_DestroyActor`))

(fn `UserConstructionScript`)