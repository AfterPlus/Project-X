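; BP_Explosive_Nade is a grenade actor that detonates on a short timer started at BeginPlay.
; Detonation spawns an explosion emitter, sets a brief remaining lifespan and overrides the static mesh's velocity along the forward vector of the player character's mesh, cached at BeginPlay.
; The RadialForce impulse is disconnected, and the graph applies no damage.
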(event `self.ReceiveBeginPlay`
  (bind (_asmaingamemode _asmainplayercontroller _asmainplayercharacter) (`BPFunctionLibrary.CastToCore_Main` self))
  (set `self.As Main Player Character` _asmainplayercharacter)
  (`KismetSystemLibrary.K2_SetTimerDelegate` (delegate `Detonate`) 2.0))

(event `Detonate`
  (`GameplayStatics.SpawnEmitterAtLocation` "/Game/StarterContent/Particles/P_Explosion.P_Explosion")
  (`self.SetLifeSpan` 3.0)
  (`PrimitiveComponent.SetPhysicsLinearVelocity` (`self.StaticMesh`) (* (`KismetMathLibrary.GetForwardVector` (`SceneComponent.K2_GetComponentRotation` (`Character.Mesh` (`self.As Main Player Character`)))) 100.0) false "None"))

(fn `UserConstructionScript`)