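; BP_StaticPulse is a grenade Blueprint with an empty Throw event, so it currently does nothing when thrown.
; An unconnected chain, which never runs, would launch the mesh along the forward vector of the GetInstance actor, adding part of that actor's velocity.
; After a short delay it would spawn explosion particles, fire a RadialForce impulse, play a sound and destroy itself.
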(event `self.Throw`)

(fn `UserConstructionScript`
  (`parent.UserConstructionScript`))