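; Enemy grenade actor that is thrown with a physics impulse, shows an area decal where it lands and explodes after a short delay.
; EnemyThrow enables mesh physics and trails, while ResetProperties restores the non-simulating state.
; A capsule overlap with a "Floor"-tagged actor halts the mesh through heavy damping, then hides it and spawns explosion particles at the actor location.
; No damage is applied here, and the decal-scaling timeline is unconnected.
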(event `self.ResetProperties`
  (bind _mesh (`self.Mesh`))
  (`PrimitiveComponent.SetSimulatePhysics` (`self.Mesh`) false)
  (`PrimitiveComponent.SetLinearDamping` _mesh 0.0)
  (`PrimitiveComponent.SetAngularDamping` _mesh 0.0)
  (`SceneComponent.SetHiddenInGame` (`self.Decal_AOI`) true false)
  (`SceneComponent.SetHiddenInGame` (`self.NS_Trails`) true false)
  (`SceneComponent.SetHiddenInGame` (`self.Mesh`) false false))

(event `self.EnemyThrow`
  (params (Impulse :type "Vector Structure"))
  (bind _mesh (`self.Mesh`))
  (`|ExecutionSequence`
    (:`then_0`
      (`SceneComponent.SetHiddenInGame` _mesh false false)
      (`PrimitiveComponent.SetSimulatePhysics` (`self.Mesh`) true)
      (`SceneComponent.SetHiddenInGame` (`self.NS_Trails`) false false))
    (:`then_1`
      (`PrimitiveComponent.AddImpulse` _mesh Impulse "None" true))))

(event `self.Capsule.OnComponentBeginOverlap`
  (params (OverlappedComponent :type "PrimitiveComponent Object Reference") (OtherActor :type "Actor Object Reference") (OtherComp :type "PrimitiveComponent Object Reference") (OtherBodyIndex :type Integer) (bFromSweep :type Boolean) (SweepResult :type "HitResult Structure (by ref)"))
  (bind _mesh (`self.Mesh`))
  (if (`self.ActorHasTag` OtherActor "Floor")
    (`PrimitiveComponent.SetLinearDamping` _mesh 1000.0)
    (`PrimitiveComponent.SetAngularDamping` _mesh 100.0)
    (`SceneComponent.SetHiddenInGame` (`self.Decal_AOI`) false false)
    (`SceneComponent.K2_SetWorldRotation` (`self.Decal_AOI`) (struct :`Pitch` -90.0) true true)
    (`SceneComponent.SetHiddenInGame` (`self.NS_Trails`) false false)
    (`KismetSystemLibrary.Delay` 2.0)
    (`SceneComponent.SetHiddenInGame` (`self.Mesh`) true false)
    (`SceneComponent.SetHiddenInGame` (`self.Decal_AOI`) true false)
    (`SceneComponent.SetHiddenInGame` (`self.NS_Trails`) true false)
    (`GameplayStatics.SpawnEmitterAtLocation` "/Game/MilitaryWeapSilver/FX/P_Grenade_Explosion_01.P_Grenade_Explosion_01" (`self.K2_GetActorLocation`))))

(fn `UserConstructionScript`)