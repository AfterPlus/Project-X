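; Enemy bullet actor that launches itself at the player as a physics-simulated projectile.
; Its AddImpulse event starts the Niagara effect, enables physics with low linear damping and applies a velocity-change impulse toward the player.
; The unnormalized offset to the player serves as the impulse, so launch speed scales with distance.
; Disconnected nodes for random cone spread and for deactivating and moving the bullet high out of the way never run.
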(event `self.AddImpulse`
  (`ActorComponent.Activate` (`self.Niagara`) false)
  (`PrimitiveComponent.SetLinearDamping` (`self.MeshComp`) 0.01)
  (`PrimitiveComponent.SetSimulatePhysics` (`self.MeshComp`) true)
  (`PrimitiveComponent.AddImpulse` (`self.MeshComp`) (- (`self.K2_GetActorLocation` (`GameplayStatics.GetPlayerCharacter` 0)) (`self.K2_GetActorLocation`)) "None" true))

(fn `UserConstructionScript`)