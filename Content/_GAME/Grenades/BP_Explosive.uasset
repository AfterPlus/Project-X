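; BP_Explosive is a thrown grenade that explodes on contact with actors tagged Floor or Enemy.
; Throw launches the mesh along the forward vector of the GetInstance actor, plus a fraction of its velocity.
; On impact it plays effects, sound and camera shake, then expands the DamageRadius sphere and destroys itself.
; That expansion triggers overlaps, which damage each BP_MasterEnemy caught and fire a radial force impulse.
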(event `self.Throw`
  (bind _returnvalue (`MyCharacter.GetInstance`))
  (`PrimitiveComponent.AddImpulse` (`self.Mesh`) (+ (* (`self.GetActorForwardVector` _returnvalue) 500.0) (/ (`self.GetVelocity` _returnvalue) 20.0)) "None" true))

(event `self.Capsule.OnComponentBeginOverlap`
  (params (OverlappedComponent :type "PrimitiveComponent Object Reference") (OtherActor :type "Actor Object Reference") (OtherComp :type "PrimitiveComponent Object Reference") (OtherBodyIndex :type Integer) (bFromSweep :type Boolean) (SweepResult :type "HitResult Structure (by ref)"))
  (if (or (`self.ActorHasTag` OtherActor "Floor") (`self.ActorHasTag` OtherActor "Enemy"))
    (`PrimitiveComponent.SetCollisionEnabled` (`self.Capsule`) "NoCollision")
    (`GameplayStatics.SpawnEmitterAtLocation` "/Game/MilitaryWeapSilver/FX/P_Grenade_Explosion_01.P_Grenade_Explosion_01" (`self.K2_GetActorLocation`))
    (`GameplayStatics.PlaySoundAtLocation` "/Game/MilitaryWeapSilver/Sound/GrenadeLauncher/Cues/GrenadeLauncher_Explosion_Cue.GrenadeLauncher_Explosion_Cue" (`self.K2_GetActorLocation`) (struct) 1.0 1.0 0.0 null null null null)
    (`SphereComponent.SetSphereRadius` (`self.Damage Radius`) 350.0 true)
    (`GameplayStatics.PlayWorldCameraShake` "/Game/_GAME/Others/BP_LPSP_CS_Explosive.BP_LPSP_CS_Explosive_C" (`self.K2_GetActorLocation`) 0.0 2000.0)
    (`self.K2_DestroyActor`)))

(event `self.Damage Radius.OnComponentBeginOverlap`
  (params (OverlappedComponent :type "PrimitiveComponent Object Reference") (OtherActor :type "Actor Object Reference") (OtherComp :type "PrimitiveComponent Object Reference") (OtherBodyIndex :type Integer) (bFromSweep :type Boolean) (SweepResult :type "HitResult Structure (by ref)"))
  (bind _asbp_master_enemy (cast `/Game/_GAME/Enemies/BP_MasterEnemy` OtherActor))
  (`ActorInterface.ApplyDamageToEnemy` _asbp_master_enemy 50.0)
  (`RadialForceComponent.FireImpulse` (`self.RadialForce`)))

(fn `UserConstructionScript`
  (`parent.UserConstructionScript`))