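; Procedural-level door that triggers alley spawning when opened and raises its mesh if CanOpen is set.
; A trigger box registers the door on BP_Character during overlap and clears it on exit.
; OpenDoorBP calls SpawnAlley, which caches the level generator and defers to the parent implementation, then runs a timeline lifting the mesh from its current height.
; An unconnected Blueprint version of alley placement with overlap checks remains in the graph.
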(event `Open Door BP`
  (bind (_returnvalue_x _returnvalue_y _returnvalue_z) (`KismetMathLibrary.BreakVector` (`SceneComponent.K2_GetComponentLocation` (`self.StaticMesh`))))
  (bind (_returnvalue_x_2 _returnvalue_y_2 _returnvalue_z_2) (`KismetMathLibrary.BreakVector` (`SceneComponent.K2_GetComponentLocation` (`self.StaticMesh`))))
  (`self.SpawnAlley`)
  (if (`self.bCanOpen`)
    (bind (_direction _alpha) (`Timeline|Timeline` :!via `PlayFromStart`)
      (:`Update`
        (`SceneComponent.K2_SetWorldLocation` (`self.StaticMesh`) (`KismetMathLibrary.MakeVector` _returnvalue_x_2 _returnvalue_y_2 (`KismetMathLibrary.Lerp` _returnvalue_z_2 (+ _returnvalue_z 10.0) _alpha)) false false)))))

(event `self.Box.OnComponentBeginOverlap`
  (params (OverlappedComponent :type "PrimitiveComponent Object Reference") (OtherActor :type "Actor Object Reference") (OtherComp :type "PrimitiveComponent Object Reference") (OtherBodyIndex :type Integer) (bFromSweep :type Boolean) (SweepResult :type "HitResult Structure (by ref)"))
  (bind _asbp_character (cast `/Game/_GAME/Player/BP_Character` OtherActor))
  (set `/Game/_GAME/Player/BP_Character.Door BP test` self _asbp_character))

(event `self.SpawnAlley`
  (bind _returnvalue (`GameplayStatics.GetActorOfClass` "/Game/_GAME/Procedural_Level/BP_LevelGenerator.BP_LevelGenerator_C"))
  (set `self.LevelGenerator` _returnvalue)
  (`parent.SpawnAlley`))

(event `self.Box.OnComponentEndOverlap`
  (params (OverlappedComponent :type "PrimitiveComponent Object Reference") (OtherActor :type "Actor Object Reference") (OtherComp :type "PrimitiveComponent Object Reference") (OtherBodyIndex :type Integer))
  (bind _asbp_character (cast `/Game/_GAME/Player/BP_Character` OtherActor))
  (set `/Game/_GAME/Player/BP_Character.Door BP test` null _asbp_character))

(fn `UserConstructionScript`)