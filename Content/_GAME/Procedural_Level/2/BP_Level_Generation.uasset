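; BP_Level_Generation is a procedural level generator that spawns a starting room and further random rooms at BeginPlay.
; It caches the starting room's exit components, but the short spawn loop passes a separate ExitPoint variable, never set here, as the transform target.
; Rooms come from a shared instance's Rooms list, with a Remove after each spawn.
; Random is evaluated separately for each use, so the removed entry can differ from the spawned one.
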(event `Spawn Start Room`
  (bind _returnvalue (`|SpawnActorFromClass` "/Game/_GAME/Procedural_Level/2/BP_StartingRoom.BP_StartingRoom_C" (`KismetMathLibrary.MakeTransform` (0.0 0.0 0.0)) "Undefined" "MultiplyWithRoot" null null))
  (set `self.ExitsPoints` (`SceneComponent.GetChildrenComponents` (`/Game/_GAME/Procedural_Level/2/BP_Room_Base.Exits` _returnvalue) false)))

(event `Spawn Next Room`
  (params (Target :type "SceneComponent Object Reference"))
  (bind (_returnvalue_location _returnvalue_rotation) (`KismetMathLibrary.BreakTransform` (`SceneComponent.K2_GetComponentToWorld` Target)))
  (bind _outitem (`KismetArrayLibrary.Array_Random` (`GameInstanceBase.Rooms` (`GameInstanceBase.GetInstance`))))
  (`|SpawnActorFromClass` _outitem (`KismetMathLibrary.MakeTransform` _returnvalue_location _returnvalue_rotation) "Undefined" "MultiplyWithRoot" null null)
  (`KismetArrayLibrary.Array_RemoveItem` (`GameInstanceBase.Rooms` (`GameInstanceBase.GetInstance`)) _outitem))

(event `self.ReceiveBeginPlay`
  (`self.Spawn Start Room`)
  (for _ (range 2)
    (`self.Spawn Next Room` (`self.ExitPoint`))))

(fn `UserConstructionScript`)