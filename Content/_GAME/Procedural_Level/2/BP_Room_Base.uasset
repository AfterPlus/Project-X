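; BP_Room_Base is a room actor for procedural level generation that attaches an alley at one of its exits.
; On BeginPlay it spawns a random class from the game instance's Alleys list at the transform of an indexed child of Exits.
; It then removes a Random result from that shared list; because Random is pure and re-evaluated, the removed entry can differ from the spawned one.
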(event `self.ReceiveBeginPlay`
  (bind _outitem (`KismetArrayLibrary.Array_Random` (`GameInstanceBase.Alleys` (`GameInstanceBase.GetInstance`))))
  (bind (_returnvalue_location _returnvalue_rotation) (`KismetMathLibrary.BreakTransform` (`SceneComponent.K2_GetComponentToWorld` (`SceneComponent.GetChildComponent` (`self.Exits`) (`self.Child Index`)))))
  (`|SpawnActorFromClass` _outitem (`KismetMathLibrary.MakeTransform` _returnvalue_location _returnvalue_rotation) "Undefined" "MultiplyWithRoot" null null)
  (`KismetArrayLibrary.Array_RemoveItem` (`GameInstanceBase.Alleys` (`GameInstanceBase.GetInstance`)) _outitem))

(fn `UserConstructionScript`)