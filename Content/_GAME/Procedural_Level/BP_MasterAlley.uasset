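; BP_MasterAlley is a procedural-level alley piece that attaches a room at its Arrow and can be parked far below the world.
; SpawnRoom tries random rooms from a shared SpawnedRooms pool, testing each raised above the Arrow for overlap before aligning it, enabling physics and removing it from the pool.
; CheckForAlleyOverlap detects collisions with downward traces from child points.
; Prop physics starts disabled and is toggled through SimulatePhysics.
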(event `self.ReceiveBeginPlay`
  (`self.SimulatePhysics` false))

(event `self.SimulatePhysics`
  (params (Simulate :type Boolean))
  (`parent.SimulatePhysics` Simulate)
  (for _array_element (`SceneComponent.GetChildrenComponents` (`self.PhysicsProps`) false)
    (bind _asstatic_mesh_component (cast `StaticMeshComponent` _array_element))
    (`PrimitiveComponent.SetSimulatePhysics` _asstatic_mesh_component Simulate)))

(event `Send To Default Location BP`
  (`self.K2_SetActorLocation` (0.0 0.0 -10000.0)))

(event `self.SpawnRoom`
  (bind _currentroom (`self.CurrentRoom`))
  (bind _currentroom_2 (`self.CurrentRoom`))
  (bind (_returnvalue_roll _returnvalue_pitch _returnvalue_yaw) (`KismetMathLibrary.BreakRotator` (`SceneComponent.K2_GetComponentRotation` (`self.Arrow`))))
  (for _ (range (+ (`KismetArrayLibrary.Array_Length` (`MainGameModeBase.SpawnedRooms` (`MainGameModeBase.GetInstance`))) 1))
    (bind _output_get (set `self.CurrentRoom` (`KismetArrayLibrary.Array_Random` (`MainGameModeBase.SpawnedRooms` (`MainGameModeBase.GetInstance`)))))
    (`/Engine/EditorBlueprintResources/StandardMacros.IsValid` _output_get
      (:`Is Valid`
        (`self.K2_SetActorLocation` _currentroom_2 (+ (`SceneComponent.K2_GetComponentLocation` (`self.Arrow`)) (0.0 0.0 500.0)) false false)
        (bind _returnvalue (`Room.CheckForRoomOverlap` _currentroom_2))
        (if _returnvalue
          (`self.K2_SetActorLocation` (`self.CurrentRoom`) (0.0 0.0 -10000.0) false false)
          (else
            (break))))))
  (`/Engine/EditorBlueprintResources/StandardMacros.IsValid` _currentroom
    (:`Is Valid`
      (`self.K2_SetActorLocation` _currentroom (`SceneComponent.K2_GetComponentLocation` (`self.Arrow`)) false false)
      (`self.K2_SetActorRotation` (`self.CurrentRoom`) (`KismetMathLibrary.MakeRotator` _returnvalue_roll _returnvalue_pitch (- _returnvalue_yaw 90.0)) false)
      (`KismetSystemLibrary.Delay` 0.2)
      (`Room.SimulatePhysics` (`self.CurrentRoom`) true)
      (`KismetArrayLibrary.Array_RemoveItem` (`MainGameModeBase.SpawnedRooms` (`MainGameModeBase.GetInstance`)) (`self.CurrentRoom`)))))

(fn `CheckForAlleyOverlap`
  (returns (ReturnValue :type Boolean))
  (locals (bIsBlocking :type Boolean :default false))
  (for _array_element (`SceneComponent.GetChildrenComponents` (`self.LineTracePoints`) false)
    (bind _returnvalue (`SceneComponent.K2_GetComponentLocation` _array_element))
    (bind _outhit (`KismetSystemLibrary.LineTraceSingle` :`Start` _returnvalue :`End` (+ _returnvalue (0.0 0.0 -1000.0)) :`TraceChannel` "TraceTypeQuery1" :`bTraceComplex` true :`DrawDebugType` "Persistent"))
    (bind _bblockinghit (`GameplayStatics.BreakHitResult` _outhit))
    (if _bblockinghit
      (return _bblockinghit)))
  (return false))

(fn `UserConstructionScript`)