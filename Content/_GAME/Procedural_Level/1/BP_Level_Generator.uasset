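; Procedural level generator actor that builds a level from random room Blueprints on BeginPlay, starting from BP_Room_1.
; Each next room spawns at a random exit from a growing list, then after a short delay its overlap boxes are tested.
; Overlapping rooms are destroyed and retried, while clear ones add their exits and decrement RoomAmount until none remain.
; A similar alley spawn-and-check path exists but is not connected to the running flow.
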(event `Spawn Start Room`
  ;[1 1 1] Spawn Start Room
  (bind _returnvalue (`|SpawnActorFromClass` "/Game/_GAME/Procedural_Level/1/BP_Room_1.BP_Room_1_C" (`KismetMathLibrary.MakeTransform` (0.0 0.0 0.0)) "AlwaysSpawn" "MultiplyWithRoot" null null))
  (bind _output_get (set `self.Latest Room` _returnvalue))
  (`KismetArrayLibrary.Array_Append` (`self.Exits List`) (`SceneComponent.GetChildrenComponents` (`/Game/_GAME/Procedural_Level/1/BP_MasterRoom.Exit` _output_get) false)))

(event `Spawn Next Room`
  (bind (_returnvalue_location _returnvalue_rotation) (`KismetMathLibrary.BreakTransform` (`SceneComponent.K2_GetComponentToWorld` (`self.Selected Exit Point`))))
  ;[1 1 1] Spawn Next Room
  (set `self.Selected Exit Point` (`KismetArrayLibrary.Array_Random` (`self.Exits List`)))
  (bind _returnvalue (`|SpawnActorFromClass` (`KismetArrayLibrary.Array_Random` (`self.Rooms List`)) (`KismetMathLibrary.MakeTransform` _returnvalue_location _returnvalue_rotation) "AlwaysSpawn" "MultiplyWithRoot" null null))
  (bind _asbp_master_room (cast `/Game/_GAME/Procedural_Level/1/BP_MasterRoom` _returnvalue))
  (set `self.Latest Room` _asbp_master_room)
  (`KismetSystemLibrary.Delay` 0.2)
  (`self.Check for Room overlap`))

(event `self.ReceiveBeginPlay`
  (`self.Spawn Start Room`)
  (`self.Spawn Next Room`))

(event `Check for Room overlap`
  (for _array_element (`SceneComponent.GetChildrenComponents` (`/Game/_GAME/Procedural_Level/1/BP_MasterRoom.OverlapFolder` (`self.Latest Room`)) false)
    (bind _asbox_collision (cast `BoxComponent` _array_element))
    (`KismetArrayLibrary.Array_Append` (`self.Overlapped List`) (`PrimitiveComponent.GetOverlappingComponents` _asbox_collision)))
  (if (`KismetArrayLibrary.Array_IsEmpty` (`self.Overlapped List`))
    (`KismetArrayLibrary.Array_Clear` (`self.Overlapped List`))
    (set `self.Room Amount` (- (`self.Room Amount`) 1))
    (`KismetArrayLibrary.Array_Append` (`self.Exits List`) (`SceneComponent.GetChildrenComponents` (`/Game/_GAME/Procedural_Level/1/BP_MasterRoom.Exit` (`self.Latest Room`)) false))
    (if (> (`self.Room Amount`) 0)
      (`self.Spawn Next Room`))
    (else
      (`KismetArrayLibrary.Array_Clear` (`self.Overlapped List`))
      (`self.K2_DestroyActor` (`self.Latest Room`))
      (`self.Spawn Next Room`))))

(event `Spawn Next Alley`
  (bind (_returnvalue_location _returnvalue_rotation) (`KismetMathLibrary.BreakTransform` (`SceneComponent.K2_GetComponentToWorld` (`self.Selected Exit Point`))))
  (set `self.Selected Exit Point` (`KismetArrayLibrary.Array_Random` (`self.Exits List`)))
  (bind _returnvalue (`|SpawnActorFromClass` (`KismetArrayLibrary.Array_Random` (`self.Alleys List`)) (`KismetMathLibrary.MakeTransform` _returnvalue_location _returnvalue_rotation) "AlwaysSpawn" "MultiplyWithRoot" null null))
  (bind _asbp_master_room (cast `/Game/_GAME/Procedural_Level/1/BP_MasterRoom` _returnvalue))
  (set `self.As Latest Alley ` _asbp_master_room)
  (`self.Check for Allay Ovelap`))

(event `Check for Allay Ovelap`
  (for _array_element (`SceneComponent.GetChildrenComponents` (`/Game/_GAME/Procedural_Level/1/BP_MasterRoom.OverlapFolder` (`self.As Latest Alley `)) false)
    (bind _asbox_collision (cast `BoxComponent` _array_element))
    (`KismetArrayLibrary.Array_Append` (`self.Overlapped List`) (`PrimitiveComponent.GetOverlappingComponents` _asbox_collision)))
  (if (`KismetArrayLibrary.Array_IsEmpty` (`self.Overlapped List`))
    (`KismetArrayLibrary.Array_Clear` (`self.Overlapped List`))
    (set `self.Selected Exit Point` (`SceneComponent.GetChildComponent` (`/Game/_GAME/Procedural_Level/1/BP_MasterRoom.Exit` (`self.As Latest Alley `)) 0))
    (`self.Spawn Next Room`)
    (else
      (`KismetArrayLibrary.Array_Clear` (`self.Overlapped List`))
      (`self.K2_DestroyActor` (`self.Latest Room`))
      (`self.Spawn Next Alley`))))

(fn `UserConstructionScript`)