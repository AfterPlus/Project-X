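; BP_MasterRoom is a room actor for procedural levels, providing doors, prop physics, an overlap check and an enemy spawn trigger.
; On BeginPlay it spawns and attaches a BP_Door at each child of Doors.
; When MyCharacter enters BoxComp, it registers as the shared instance's CurrentRoom and requests enemy deployment at a random spawn point.
; CheckForRoomOverlap traces downward from marker components, while SimulatePhysics toggles physics on prop meshes.
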(event `self.SimulatePhysics`
  (params (Simulate :type Boolean))
  (for _array_element (`SceneComponent.GetChildrenComponents` (`self.PhysicsProps`) false)
    (bind _asstatic_mesh_component (cast `StaticMeshComponent` _array_element))
    (`PrimitiveComponent.SetSimulatePhysics` _asstatic_mesh_component Simulate)))

(event `self.ReceiveBeginPlay`
  (for _array_element (`SceneComponent.GetChildrenComponents` (`self.Doors`) false)
    (bind _returnvalue (`|SpawnActorFromClass` "/Game/_GAME/Procedural_Level/BP_Door.BP_Door_C" (`KismetMathLibrary.MakeTransform` (0.0 0.0 0.0)) "Undefined" "MultiplyWithRoot" null null))
    (`KismetArrayLibrary.Array_Add` (`self.SpawnedDoors`) _returnvalue)
    (`self.K2_AttachToComponent` _returnvalue _array_element "None" "SnapToTarget" "SnapToTarget" "SnapToTarget" true)))

(event `self.BoxComp.OnComponentBeginOverlap`
  (params (OverlappedComponent :type "PrimitiveComponent Object Reference") (OtherActor :type "Actor Object Reference") (OtherComp :type "PrimitiveComponent Object Reference") (OtherBodyIndex :type Integer) (bFromSweep :type Boolean) (SweepResult :type "HitResult Structure (by ref)"))
  (bind _outitem (`KismetArrayLibrary.Array_Random` (`SceneComponent.GetChildrenComponents` (`self.EnemiesSpawnPoints`) true)))
  (cast `MyCharacter` OtherActor)
  (set `MainGameModeBase.CurrentRoom` self (`MainGameModeBase.GetInstance`))
  (bind _returnvalue (`LevelManager.GetInstance`))
  (`/Engine/EditorBlueprintResources/StandardMacros.IsValid` _outitem
    (:`Is Valid`
      (`LevelManager.DeployEnemies` _returnvalue (`SceneComponent.K2_GetComponentLocation` _outitem)))))

(fn `CheckForRoomOverlap`
  (returns (ReturnValue :type Boolean))
  (for _array_element (`SceneComponent.GetChildrenComponents` (`self.LineTracePoints`) false)
    (bind _returnvalue (`SceneComponent.K2_GetComponentLocation` _array_element))
    (bind _outhit (`KismetSystemLibrary.LineTraceSingle` :`Start` _returnvalue :`End` (+ _returnvalue (0.0 0.0 -1000.0)) :`TraceChannel` "TraceTypeQuery1" :`DrawDebugType` "Persistent"))
    (if (`GameplayStatics.BreakHitResult` _outhit)
      (return true)))
  (return false))

(fn `UserConstructionScript`)