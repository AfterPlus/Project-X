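; BP_LevelGenerator builds the pool of room and alley actors for a procedural level.
; On BeginPlay it spawns one actor per class in Rooms and Alleys at fixed points below the origin, passing itself as LevelGenerator.
; The instances are stored in SpawnedRooms and SpawnedAlley.
; Logic to move a random room to the generator and remove it from the pool exists but is unconnected.
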(event `Store all the rooms`
  (for _array_element (`self.Rooms`)
    (bind _returnvalue (`|SpawnActorFromClass` _array_element (`KismetMathLibrary.MakeTransform` (0.0 0.0 -1000.0)) "Undefined" "MultiplyWithRoot" null self null))
    (`KismetArrayLibrary.Array_AddUnique` (`self.Spawned Rooms`) _returnvalue)))

(event `Store all Alley`
  (for _array_element (`self.Alleys`)
    (bind _returnvalue (`|SpawnActorFromClass` _array_element (`KismetMathLibrary.MakeTransform` (0.0 -1000.0 -1000.0)) "Undefined" "MultiplyWithRoot" null self null))
    (`KismetArrayLibrary.Array_Add` (`self.Spawned Alley`) _returnvalue)))

(event `self.ReceiveBeginPlay`
  (`self.Store all the rooms`)
  (`self.Store all Alley`))

(fn `UserConstructionScript`)