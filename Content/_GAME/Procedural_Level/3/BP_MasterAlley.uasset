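; Base alley piece for procedural level generation that attaches rooms from the LevelGenerator's pool of already-spawned rooms.
; SpawnRooms test-places random rooms above its Arrow, sending overlapping ones far below the map, then snaps the last pick to the Arrow, enables its physics and removes it from the pool.
; CheckIfOverlap detects blockers with debug-drawn downward traces from LineTracePoints children; helpers toggle mesh physics and park the alley below the map.
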(event `self.ReceiveBeginPlay`)

(event `Send To Default Location`
  (`self.K2_SetActorLocation` (0.0 0.0 -10000.0)))

(event `Set Simulate Physics`
  (params (bSimulate :type Boolean))
  (for _array_element (`SceneComponent.GetChildrenComponents` (`self.Physics`) false)
    (bind _asstatic_mesh_component (cast `StaticMeshComponent` _array_element))
    (`PrimitiveComponent.SetSimulatePhysics` _asstatic_mesh_component bSimulate)))

(event `Spawn Rooms`
  (params (Door :type "/Game/_GAME/Procedural_Level/3/BP_Door Object Reference"))
  (bind _spawned_room (`self.Spawned Room`))
  (bind (_returnvalue_roll _returnvalue_pitch _returnvalue_yaw) (`KismetMathLibrary.BreakRotator` (`SceneComponent.K2_GetComponentRotation` (`self.Arrow`))))
  (`KismetSystemLibrary.Delay` 0.2)
  (for _ (range (`KismetArrayLibrary.Array_Length` (`/Game/_GAME/Procedural_Level/3/BP_LevelGenerator.Spawned Rooms` (`self.Level Generator`))))
    (bind _output_get (set `self.Spawned Room` (`KismetArrayLibrary.Array_Random` (`/Game/_GAME/Procedural_Level/3/BP_LevelGenerator.Spawned Rooms` (`self.Level Generator`)))))
    (`/Engine/EditorBlueprintResources/StandardMacros.IsValid` _output_get
      (:`Is Valid`
        (`self.K2_SetActorLocation` _output_get (+ (`SceneComponent.K2_GetComponentLocation` (`self.Arrow`)) (0.0 0.0 500.0)) false false)
        (if (`/Game/_GAME/Procedural_Level/3/BP_MasterRoom.Check for Overlap` (`self.Spawned Room`))
          (`/Game/_GAME/Procedural_Level/3/BP_MasterRoom.Send To Default Location` (`self.Spawned Room`))
          (else
            (break))))))
  (`/Engine/EditorBlueprintResources/StandardMacros.IsValid` _spawned_room
    (:`Is Valid`
      (`self.K2_SetActorLocation` _spawned_room (`SceneComponent.K2_GetComponentLocation` (`self.Arrow`)) false false)
      (`self.K2_SetActorRotation` (`self.Spawned Room`) (`KismetMathLibrary.MakeRotator` _returnvalue_roll _returnvalue_pitch (- _returnvalue_yaw 90.0)) false)
      (`KismetSystemLibrary.Delay` 0.2)
      (`/Game/_GAME/Procedural_Level/3/BP_MasterRoom.Set Simulate Physics` (`self.Spawned Room`) true)
      (`KismetArrayLibrary.Array_RemoveItem` (`/Game/_GAME/Procedural_Level/3/BP_LevelGenerator.Spawned Rooms` (`self.Level Generator`)) (`self.Spawned Room`)))))

(fn `Check If Overlap`
  (returns (Return :type Boolean))
  (for _array_element (`SceneComponent.GetChildrenComponents` (`self.Line trace points`) false)
    (bind _returnvalue (`SceneComponent.K2_GetComponentLocation` _array_element))
    (bind _outhit (`KismetSystemLibrary.LineTraceSingle` :`Start` _returnvalue :`End` (+ _returnvalue (0.0 0.0 -1000.0)) :`TraceChannel` "TraceTypeQuery1" :`bTraceComplex` true :`DrawDebugType` "Persistent"))
    (bind _bblockinghit (`GameplayStatics.BreakHitResult` _outhit))
    (if _bblockinghit
      (return _bblockinghit)))
  (return false))

(fn `UserConstructionScript`)