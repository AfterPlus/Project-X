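; BP_MasterRoom is a room actor for procedural level generation, likely the base for level pieces.
; On BeginPlay it spawns a BP_Door at each child of its Door component, attaches it and passes on the LevelGenerator.
; CheckForOverlap traces downward from each LineTrace child, drawing persistent debug lines, and returns true on the first blocking hit.
; Events toggle physics on meshes under Physics and move the room far below the origin.
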(event `Set Simulate Physics`
  (params (bSimulate :type Boolean))
  (for _array_element (`SceneComponent.GetChildrenComponents` (`self.Physics`) false)
    (bind _asstatic_mesh_component (cast `StaticMeshComponent` _array_element))
    (`PrimitiveComponent.SetSimulatePhysics` _asstatic_mesh_component bSimulate)))

(event `self.ReceiveBeginPlay`
  (for _array_element (`SceneComponent.GetChildrenComponents` (`self.Door`) false)
    (bind _returnvalue (`|SpawnActorFromClass` "/Game/_GAME/Procedural_Level/3/BP_Door.BP_Door_C" (`KismetMathLibrary.MakeTransform` (0.0 0.0 0.0)) "Undefined" "MultiplyWithRoot" null (`self.Level Generator`) null))
    (`self.K2_AttachToComponent` _returnvalue _array_element "None" "SnapToTarget" "SnapToTarget" "SnapToTarget" true)))

(event `Send To Default Location`
  (`self.K2_SetActorLocation` (0.0 0.0 -10000.0)))

(fn `Check for Overlap`
  (returns (Return :type Boolean))
  (locals (`Blocking Hit` :type Boolean))
  (for _array_element (`SceneComponent.GetChildrenComponents` (`self.Line Trace`) false)
    (bind _returnvalue (`SceneComponent.K2_GetComponentLocation` _array_element))
    (bind _outhit (`KismetSystemLibrary.LineTraceSingle` :`Start` _returnvalue :`End` (+ _returnvalue (0.0 0.0 -1000.0)) :`TraceChannel` "TraceTypeQuery1" :`DrawDebugType` "Persistent"))
    (bind _bblockinghit (`GameplayStatics.BreakHitResult` _outhit))
    (set `local.Blocking Hit` _bblockinghit)
    (if _bblockinghit
      (return (`local.Blocking Hit`))))
  (return false))

(fn `UserConstructionScript`)