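; Procedural-level door that grows the level when opened, registering itself with BP_Character through box overlap.
; OpenDoor starts SpawnAlley and, if CanOpen, raises the mesh by Timeline.
; After a delay, SpawnAlley tests random alleys from BP_LevelGenerator's pre-spawned pool above the door, returning overlapping ones and clearing CanOpen.
; If CanOpen holds, the alley moves to the door, enables physics, spawns rooms and leaves the pool.
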(event `Open Door`
  (bind (_returnvalue_x _returnvalue_y _returnvalue_z) (`KismetMathLibrary.BreakVector` (`SceneComponent.K2_GetComponentLocation` (`self.StaticMesh`))))
  (bind (_returnvalue_x_2 _returnvalue_y_2 _returnvalue_z_2) (`KismetMathLibrary.BreakVector` (`SceneComponent.K2_GetComponentLocation` (`self.StaticMesh`))))
  (`self.Spawn Alley`)
  (if (`self.Can Open`)
    (bind (_direction _alpha) (`Timeline|Timeline` :!via `PlayFromStart`)
      (:`Update`
        (`SceneComponent.K2_SetWorldLocation` (`self.StaticMesh`) (`KismetMathLibrary.MakeVector` _returnvalue_x_2 _returnvalue_y_2 (`KismetMathLibrary.Lerp` _returnvalue_z_2 (+ _returnvalue_z 10.0) _alpha)) false false)))))

(event `self.ReceiveBeginPlay`
  (bind _returnvalue (`GameplayStatics.GetActorOfClass` "/Game/_GAME/Procedural_Level/3/BP_LevelGenerator.BP_LevelGenerator_C"))
  (set `self.Level Generator` _returnvalue))

(event `Spawn Alley`
  (bind _spawned_alley (`self.Spawned Alley`))
  (`KismetSystemLibrary.Delay` 0.2)
  (for _ (range (+ (`KismetArrayLibrary.Array_Length` (`/Game/_GAME/Procedural_Level/3/BP_LevelGenerator.Spawned Alley` (`self.Level Generator`))) 1))
    (bind _output_get (set `self.Spawned Alley` (`KismetArrayLibrary.Array_Random` (`/Game/_GAME/Procedural_Level/3/BP_LevelGenerator.Spawned Alley` (`self.Level Generator`)))))
    (`/Engine/EditorBlueprintResources/StandardMacros.IsValid` _output_get
      (:`Is Valid`
        (`self.K2_SetActorLocation` _spawned_alley (+ (`self.K2_GetActorLocation`) (0.0 0.0 500.0)) false false)
        (`self.K2_SetActorRotation` _spawned_alley (`self.K2_GetActorRotation`) false)
        (bind _asbp_master_alley (cast `/Game/_GAME/Procedural_Level/3/BP_MasterAlley` (`self.Spawned Alley`)))
        (if (`/Game/_GAME/Procedural_Level/3/BP_MasterAlley.Check If Overlap` _asbp_master_alley)
          (bind _asbp_master_alley_2 (cast `/Game/_GAME/Procedural_Level/3/BP_MasterAlley` (`self.Spawned Alley`)))
          (`/Game/_GAME/Procedural_Level/3/BP_MasterAlley.Send To Default Location` _asbp_master_alley_2)
          (set `self.Can Open` false)
          (else
            (break))))))
  (if (`self.Can Open`)
    (`self.K2_SetActorLocation` (`self.Spawned Alley`) (`self.K2_GetActorLocation`) false false)
    (bind _asbp_master_alley_3 (cast `/Game/_GAME/Procedural_Level/3/BP_MasterAlley` (`self.Spawned Alley`)))
    (`KismetSystemLibrary.Delay` 0.2)
    (`/Game/_GAME/Procedural_Level/3/BP_MasterAlley.Set Simulate Physics` _asbp_master_alley_3 true)
    (bind _asbp_master_alley_4 (cast `/Game/_GAME/Procedural_Level/3/BP_MasterAlley` (`self.Spawned Alley`)))
    (`/Game/_GAME/Procedural_Level/3/BP_MasterAlley.Spawn Rooms` _asbp_master_alley_4 self)
    (`KismetArrayLibrary.Array_RemoveItem` (`/Game/_GAME/Procedural_Level/3/BP_LevelGenerator.Spawned Alley` (`self.Level Generator`)) _asbp_master_alley_4)
    (set `self.Can Open` true)))

(event `self.Box.OnComponentBeginOverlap`
  (params (OverlappedComponent :type "PrimitiveComponent Object Reference") (OtherActor :type "Actor Object Reference") (OtherComp :type "PrimitiveComponent Object Reference") (OtherBodyIndex :type Integer) (bFromSweep :type Boolean) (SweepResult :type "HitResult Structure (by ref)"))
  (bind _asbp_character (cast `/Game/_GAME/Player/BP_Character` OtherActor))
  (set `/Game/_GAME/Player/BP_Character.Door BP test` self _asbp_character))

(event `self.Box.OnComponentEndOverlap`
  (params (OverlappedComponent :type "PrimitiveComponent Object Reference") (OtherActor :type "Actor Object Reference") (OtherComp :type "PrimitiveComponent Object Reference") (OtherBodyIndex :type Integer))
  (bind _asbp_character (cast `/Game/_GAME/Player/BP_Character` OtherActor))
  (set `/Game/_GAME/Player/BP_Character.Door BP test` null _asbp_character))

(fn `UserConstructionScript`)