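; BP_LootCrate is an interactable loot crate that plays an opening animation and spawns pickups.
; A sphere overlap starts or stops interaction on BP_Character, and leaving also hides the widget and custom-depth highlight.
; OpenCrateBP repeatedly spawns every Resources class, plus one BP_WeaponLoot, at SpawnPoint.
; Its IsOpen guard sets the flag to false, so this graph never blocks reopening.
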(event `Open Crate BP`
  (if (not (`self.bIsOpen`))
    (set `self.bIsOpen` false)
    (`SkeletalMeshComponent.PlayAnimation` (`self.SkeletalMesh`) "/Game/_GAME/LootCrate/Mesh/military_crate/sci-fi_crate/sci-fi-crate/source/A_CrateOpening.A_CrateOpening" false)
    (for _ (range 3)
      (for _array_element (`self.Resources`)
        (`|SpawnActorFromClass` _array_element (`KismetMathLibrary.MakeTransform` (`SceneComponent.K2_GetComponentLocation` (`self.SpawnPoint`))) "Undefined" "OverrideRootScale" null (`self.GetActorForwardVector`) null)))
    (`|SpawnActorFromClass` "/Game/_GAME/Resources/BP_WeaponLoot.BP_WeaponLoot_C" (`KismetMathLibrary.MakeTransform` (`SceneComponent.K2_GetComponentLocation` (`self.SpawnPoint`))) "Undefined" "OverrideRootScale" null (`self.GetActorForwardVector`) null)))

(event `self.Sphere.OnComponentBeginOverlap`
  (params (OverlappedComponent :type "PrimitiveComponent Object Reference") (OtherActor :type "Actor Object Reference") (OtherComp :type "PrimitiveComponent Object Reference") (OtherBodyIndex :type Integer) (bFromSweep :type Boolean) (SweepResult :type "HitResult Structure (by ref)"))
  (bind _asbp_character (cast `/Game/_GAME/Player/BP_Character` OtherActor))
  (`ActorInterface.StartInteract` _asbp_character self))

(event `self.Sphere.OnComponentEndOverlap`
  (params (OverlappedComponent :type "PrimitiveComponent Object Reference") (OtherActor :type "Actor Object Reference") (OtherComp :type "PrimitiveComponent Object Reference") (OtherBodyIndex :type Integer))
  (bind _asbp_character (cast `/Game/_GAME/Player/BP_Character` OtherActor))
  (`ActorInterface.StopInteract` _asbp_character self)
  (`PrimitiveComponent.SetRenderCustomDepth` (`self.SkeletalMesh`) false)
  (`SceneComponent.SetHiddenInGame` (`self.Widget`) true false))

(fn `UserConstructionScript`)