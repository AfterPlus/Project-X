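; Weapon system component that handles the character picking up weapons into a limited inventory.
; PickUpWeapon routes through a macro comparing weapon names (only the last comparison counts) and slot count to pick ammo, add or swap.
; Adding stows the held weapon on a slot and grips the new one; swapping tosses the held weapon forward and takes its array entry.
; Ammo pickup only prints; an old class-based pickup graph remains, mostly disconnected.
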(event `self.SwapWeapon`)

(event `Pick Weapon`
  (bind _interactingweapon (`self.InteractingWeapon`))
  (set `self.InHandWeapon` _interactingweapon)
  (bind _returnvalue (`GameplayStatics.GetActorOfClass` (`MasterWeapon.ClassReference` _interactingweapon))))

(event `self.PickUpWeapon`
  (params (Weapon :type "MasterWeapon Object Reference"))
  (bind _interactingweapon (`self.InteractingWeapon`))
  (bind _as_bp_character (`self.As BP Character`))
  (bind _as_bp_character_2 (`self.As BP Character`))
  (bind _as_bp_character_3 (`self.As BP Character`))
  (bind _as_bp_character_4 (`self.As BP Character`))
  (bind _inhandweapon (`MyCharacter.InHandWeapon` _as_bp_character))
  (bind _inhandweapon_2 (`MyCharacter.InHandWeapon` _as_bp_character_3))
  (`parent.PickUpWeapon` Weapon)
  (bind _output_get (set `self.InteractingWeapon` Weapon))
  (`self.Ckeck for Weapon Swap` _output_get
    (:`Pick ammo`
      (`KismetSystemLibrary.PrintString` "Pick Ammo"))
    (:`Pick Weapon`
      (if (not (< (`KismetArrayLibrary.Array_Length` (`MyCharacter.AllWeapons` (`self.As BP Character`))) 1))
        (`/Engine/EditorBlueprintResources/StandardMacros.IsValid` (`MyCharacter.InHandWeapon` (`self.As BP Character`))
          (:`Is Valid`
            (`Actor.K2_DetachFromActor` _inhandweapon "KeepWorld" "KeepWorld" "KeepWorld")
            (`MasterWeapon.UpdateWeaponState` _inhandweapon "EIR_InInventory")
            (`/Engine/EditorBlueprintResources/StandardMacros.IncrementInt` (`MyCharacter.WeaponIndex` _as_bp_character)
              (:`  `
                (`Actor.K2_AttachToComponent` (`MyCharacter.InHandWeapon` _as_bp_character_4) (`|GetArrayItem` (`MyCharacter.WeaponSlots` _as_bp_character_4) (- (`KismetArrayLibrary.Array_Length` (`MyCharacter.AllWeapons` _as_bp_character_4)) 1)) "None" "SnapToTarget" "SnapToTarget" "SnapToTarget" true))))))
      (`Actor.K2_AttachToComponent` _interactingweapon (`/Game/_GAME/Player/BP_Character.Mesh_1P` (`self.As BP Character`)) "GripPoint" "SnapToTarget" "SnapToTarget" "SnapToTarget" true)
      (`MasterWeapon.UpdateWeaponState` _interactingweapon "EIR_InHand")
      (set `MyCharacter.InHandWeapon` _interactingweapon _as_bp_character_2)
      (`/Engine/EditorBlueprintResources/StandardMacros.IncrementInt` (`MyCharacter.WeaponIndex` _as_bp_character_2)
        (:`  `
          (`KismetArrayLibrary.Array_Add` (`MyCharacter.AllWeapons` (`self.As BP Character`)) _interactingweapon))))
    (:`Swap Weapon`
      (`Actor.K2_DetachFromActor` _inhandweapon_2 "KeepWorld" "KeepWorld" "KeepWorld")
      (`MasterWeapon.UpdateWeaponState` _inhandweapon_2 "EIR_OnGround")
      (`PrimitiveComponent.SetAllPhysicsLinearVelocity` (`MasterWeapon.GunMesh` _inhandweapon_2) (* (`SceneComponent.GetForwardVector` (`Actor.RootComponent` (`self.As BP Character`))) 200.0) false)
      (`KismetArrayLibrary.Array_Set` (`MyCharacter.AllWeapons` (`self.As BP Character`)) (`KismetArrayLibrary.Array_Find` (`MyCharacter.AllWeapons` _as_bp_character_3) _inhandweapon_2) (`self.InteractingWeapon`) true)
      (`Actor.K2_AttachToComponent` (`self.InteractingWeapon`) (`/Game/_GAME/Player/BP_Character.Mesh_1P` (`self.As BP Character`)) "GripPoint" "SnapToTarget" "SnapToTarget" "SnapToTarget" true)
      (`MasterWeapon.UpdateWeaponState` (`self.InteractingWeapon`) "EIR_InHand")
      (set `MyCharacter.InHandWeapon` (`self.InteractingWeapon`) (`self.As BP Character`)))))

(fn `CheckForWeaponSwap`
  (params (Weapon :type "MasterWeapon Object Reference"))
  (returns (ReturnValue :type Boolean))
  (locals (SameWeaponTypeBP :type Boolean :default false)))