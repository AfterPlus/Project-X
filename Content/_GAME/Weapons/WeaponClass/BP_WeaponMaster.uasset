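; Base weapon actor for first-person guns that can be picked up, carried, fired and reloaded.
; Weapon state toggles collision, physics and visibility, while sphere overlap shows an interact widget and interaction calls the player's weapon system component.
; A looping timer drives auto-fire camera hitscans, with ADS and a recoil timeline shaping spread and recoil kick, but applies no damage.
; Ammo lives on the player's InHandWeapon, refills after reload montages, and shots notify the HUD through EventsHolder.
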(event `self.Reload`
  (params (ReloadMontage :type "AnimMontage Object Reference"))
  (bind _playerref (`self.PlayerRef`))
  (bind _inhandweapon (`MyCharacter.InHandWeapon` _playerref))
  (if (> (`MasterWeapon.TotalAmmo` (`MyCharacter.InHandWeapon` (`self.PlayerRef`))) 0.0)
    (set `/Game/_GAME/Player/BP_Character.CanFire BP` false (`self.PlayerRef`))
    (if (not (`MasterWeapon.bIsReloading` _inhandweapon))
      (set `MasterWeapon.bIsReloading` true _inhandweapon)
      (else
        (set `/Game/_GAME/Player/BP_Character.CanFire BP` true _playerref)))
    (`|PlayMontage` (`/Game/_GAME/Player/BP_Character.Mesh_1P` (`self.PlayerRef`)) ReloadMontage
      (:`OnCompleted`
        (`self.Update ammo when reloading`
          (:`Out`
            (set `MasterWeapon.bIsReloading` false (`MyCharacter.InHandWeapon` (`self.PlayerRef`)))
            (set `/Game/_GAME/Player/BP_Character.CanFire BP` true (`self.PlayerRef`)))))
      (:`OnInterrupted`
        (set `/Game/_GAME/Player/BP_Character.CanFire BP` true (`self.PlayerRef`))))))

(event `self.AutoReload`
  (`self.Clear Timer`)
  (`self.Reload` (`MasterWeapon.ReloadAnimation` (`MyCharacter.InHandWeapon` (`self.PlayerRef`)))))

(event `self.ReceiveBeginPlay`
  ;[1 1 1] Get Player Ref
  (bind _asbp_character (cast `/Game/_GAME/Player/BP_Character` (`GameplayStatics.GetPlayerCharacter` 0)))
  (set `self.PlayerRef` _asbp_character)
  (bind _returnvalue (`|CreateWidget` "/Game/_GAME/Widget/WBP_Interact.WBP_Interact_C" null (`self.WeaponName`)))
  (set `self.InteractiveWidget` _returnvalue)
  (`self.UpdateWeaponState` "EIR_OnGround"))

(event `Equip`
  (set `MyCharacter.ADS_Offset` (`self.ADS_Offset`) (`self.PlayerRef`)))

(event `ActorInterface.DeleteClass`
  (`self.K2_DestroyActor`))

(event `self.UpdateWeaponState`
  (params (WeaponState :type "EWeaponState Enum" :default "EIR_OnGround"))
  ;[0.5406 1 0.7476] Update weapon  state
  (switch `EWeaponState` WeaponState
    (:`EIR_OnGround`
      (`self.SetActorEnableCollision` true)
      (`PrimitiveComponent.SetSimulatePhysics` (`self.SkeletalMeshComponent`) true)
      (`self.SetActorHiddenInGame` false))
    (:`EIR_InHand`
      (`self.SetActorEnableCollision` false)
      (`PrimitiveComponent.SetSimulatePhysics` (`self.SkeletalMeshComponent`) false)
      (`self.SetActorHiddenInGame` false))
    (:`EIR_InInventory`
      (`self.SetActorEnableCollision` false)
      (`PrimitiveComponent.SetSimulatePhysics` (`self.SkeletalMeshComponent`) false)
      (`self.SetActorHiddenInGame` true))))

(event `Cancel Reload`)

(event `self.SphereComponent.OnComponentBeginOverlap`
  (params (OverlappedComponent :type "PrimitiveComponent Object Reference") (OtherActor :type "Actor Object Reference") (OtherComp :type "PrimitiveComponent Object Reference") (OtherBodyIndex :type Integer) (bFromSweep :type Boolean) (SweepResult :type "HitResult Structure (by ref)"))
  ;[0.07239 0.4598 1] Pick Up widget
  (cast `/Game/_GAME/Player/BP_Character` OtherActor)
  (bind _returnvalue (`|CreateWidget` "/Game/_GAME/Widget/WBP_Interact.WBP_Interact_C" null (`self.WeaponName`)))
  (bind _output_get (set `self.InteractiveWidget` _returnvalue))
  (`UserWidget.AddToViewport` _output_get 0))

(event `Stow`)

(event `self.SphereComponent.OnComponentEndOverlap`
  (params (OverlappedComponent :type "PrimitiveComponent Object Reference") (OtherActor :type "Actor Object Reference") (OtherComp :type "PrimitiveComponent Object Reference") (OtherBodyIndex :type Integer))
  ;[0.07239 0.4598 1] Pick Up widget
  (cast `/Game/_GAME/Player/BP_Character` OtherActor)
  (`Widget.RemoveFromParent` (stale `self.SphereComponent.OnComponentBeginOverlap` _output_get)))

(event `ActorInterface.InteractPressed`
  (params (Interact_Actor :type "Actor Object Reference"))
  ;[0.9929 1 0.487] Interact pressed Interface
  (`WeaponSystemComponent.PickUpWeapon` (`self.GetComponentByClass` Interact_Actor "/Game/_GAME/Weapons/BP_WeaponSystemCOmponent.BP_WeaponSystemComponent_C") self))

(event `ActorInterface.StartWeaponFire`
  (`self.Fire`))

(event `Fire Alpha`
  (`self.UpdatePlayerYawAndPitch` (`KismetMathLibrary.RandomFloatInRange` -4.0 0.4) (`KismetMathLibrary.RandomFloatInRange` -4.0 4.0))
  (bind (_direction _recoil_alpha) (`Timeline|Recoil Alpha` :!via `PlayFromStart` :!label _label)
    (:`Update`
      (set `self.RecoilAlpha` (* _recoil_alpha (`.Spray` (break `CharactersStats` (`MyCharacter.CharactersStats` (`self.PlayerRef`)))))))))

(event `ActorInterface.WeaponReload`
  (`self.Reload` (`MasterWeapon.ReloadAnimation` (`MyCharacter.InHandWeapon` (`self.PlayerRef`)))))

(event `Stop Fire`
  (`self.Clear Timer`)
  (set `self.Bool` true)
  (goto _label :!via `ReverseFromEnd`))

(event `ActorInterface.StopWeaponFire`
  (`self.Stop Fire`))

(event `Fire`
  (bind _inhandweapon (`MyCharacter.InHandWeapon` (`self.PlayerRef`)))
  (set `self.Bool` true)
  (if (> (`MasterWeapon.AmmoInMagazine` _inhandweapon) 0.0)
    (`self.Fire Alpha`)
    (switch `EFireMode` (`MasterWeapon.FireMode` _inhandweapon)
      (:`EIR_Auto`
        (bind _returnvalue (`KismetSystemLibrary.K2_SetTimer` self "Auto Fire" 0.15 true -0.15))))
    (else
      (`self.AutoReload`))))

(event `Clear Timer`
  (bind _output_get (set `self.AutoFire Timer` (stale `Fire` _returnvalue)))
  (`KismetSystemLibrary.K2_ClearAndInvalidateTimerHandle` _output_get))

(event `Auto Fire`
  (bind _playerref (`self.PlayerRef`))
  (bind _inhandweapon (`MyCharacter.InHandWeapon` (`self.PlayerRef`)))
  (if (`self.Bool`)
    (set `self.Bool` false)
    (if (> (`MasterWeapon.AmmoInMagazine` _inhandweapon) 0.0)
      (if (and (`/Game/_GAME/Player/BP_Character.isFiring` _playerref) (`/Game/_GAME/Player/BP_Character.CanFire BP` _playerref))
        (`self.Fire_HitScan` (`MasterWeapon.Spread` _inhandweapon))
        (`/Engine/EditorBlueprintResources/StandardMacros.DecrementFloat` (`MasterWeapon.AmmoInMagazine` (`MyCharacter.InHandWeapon` (`self.PlayerRef`)))
          (:`  `
            (`|PlayMontage` (`/Game/_GAME/Player/BP_Character.Mesh_1P` (`self.PlayerRef`)) (`self.FireAnimation`)
              (:`then`
                (`EventsHolder.PlayHUDFireAnimationReq` (`MainGameModeBase.EventsHolder` (`MainGameModeBase.GetInstance`)) (`self.WeaponTypeEnum`))
                (set `self.Bool` true)
                (`EventsHolder.PlayAmmoCountAnim` (`MainGameModeBase.EventsHolder` (`MainGameModeBase.GetInstance`)))
                (if (not (> (`MasterWeapon.AmmoInMagazine` (`MyCharacter.InHandWeapon` (`self.PlayerRef`))) 0.0))
                  (`self.AutoReload`)))))))
      (else
        (`self.AutoReload`)))))

(fn `Fire_HitScan`
  (params (Spread :type "Float (double-precision)"))
  (bind _camera (`/Game/_GAME/Player/BP_Character.Camera` (`self.PlayerRef`)))
  (bind _returnvalue (`SceneComponent.K2_GetComponentLocation` _camera))
  (bind _outhit (`KismetSystemLibrary.LineTraceSingle` _returnvalue (+ _returnvalue (* (`KismetMathLibrary.RandomUnitVectorInConeInDegrees` (`SceneComponent.GetForwardVector` _camera) (* (/ Spread (`KismetMathLibrary.MapRangeClamped` (`MyCharacter.ADSAlpha` (`self.PlayerRef`)) 0.0 1.0 1.0 1.5)) (`self.RecoilAlpha`))) 20000.0)) "TraceTypeQuery1"))
  (`self.Fire Alpha`)
  (bind (_bblockinghit _binitialoverlap _time _distance _location _impactpoint _normal) (`GameplayStatics.BreakHitResult` _outhit))
  (`GameplayStatics.SpawnEmitterAtLocation` "/Game/MilitaryWeapSilver/FX/P_Impact_Stone_Large_01.P_Impact_Stone_Large_01" _impactpoint (`KismetMathLibrary.Conv_VectorToRotator` _normal))
  (`KismetSystemLibrary.DrawDebugSphere` _impactpoint 10.0 12 (struct :`R` 1.0 :`A` 1.0) 0.0 3.0))

(fn `UpdatePlayerYawAndPitch`
  (params (Pitch :type "Float (double-precision)") (Yaw :type "Float (double-precision)"))
  (bind _returnvalue (`GameplayStatics.GetPlayerController` 0))
  (`PlayerController.AddPitchInput` _returnvalue (/ (* (`.Recoil` (break `CharactersStats` (`MyCharacter.CharactersStats` (`self.PlayerRef`)))) Pitch) 25.0))
  (`PlayerController.AddYawInput` _returnvalue (/ (* Yaw (`.Recoil` (break `CharactersStats` (`MyCharacter.CharactersStats` (`self.PlayerRef`))))) 50.0))
  (return))

(fn `UserConstructionScript`
  (`SkinnedMeshComponent.SetSkinnedAssetAndUpdate` (`self.SkeletalMeshComponent`) (`self.GunSkeletalMesh`) true)
  (`PrimitiveComponent.SetMaterial` (`self.SkeletalMeshComponent`) 0 (`self.Material`)))