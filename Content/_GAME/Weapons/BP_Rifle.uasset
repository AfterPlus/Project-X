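; Rifle weapon Blueprint that adds auto hitscan fire, montage-driven reload and camera recoil on top of its parent weapon logic.
; Auto fire loops on a short delay while shooting is allowed, and reloading exits ADS and is guarded against re-entry.
; A recoil timeline kicks pitch and yaw while firing, then reverses on stop, scaling pitch recovery by drift from the DoOnce-captured starting rotation and leaving yaw unrecovered.
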(event `self.Equip`
  (set `MyCharacter.ADS_Offset` (`self.ADS_Offset_BP`) (`self.PlayerRef`)))

(event `ActorInterface.StartWeaponFire`
  (bind _playerref (`self.PlayerRef`))
  (bind _can_fire (`self.CanShoot`))
  (if _can_fire
    (`self.Fire Start`)
    (set `/Game/_GAME/Player/BP_Character.CanShootBP` true (`self.PlayerRef`))
    (switch `EFireMode` (`self.FireMode`)
      (:`EIR_Auto`
        (bind _can_fire_2 (`self.CanShoot` :!label _label))
        (if (and _can_fire_2 (`/Game/_GAME/Player/BP_Character.CanShootBP` _playerref))
          (`self.Fire_HitScan` true (`self.Spread`))
          (`KismetSystemLibrary.Delay` 0.2)
          (`|PlayMontage` (`/Game/_GAME/Player/BP_Character.Mesh_1P` _playerref) "/Game/_GAME/ProceduralAnimation/Animations/FP_Fire_Montage.FP_Fire_Montage"
            (:`then`
              (goto _label))))))))

(event `ActorInterface.StopWeaponFire`
  (`self.Fire Stop`))

(event `ActorInterface.WeaponReload`
  (bind _playerref (`self.PlayerRef`))
  (`self.Reload`)
  (if (not (`self.bReloading ?`))
    (set `self.bReloading ?` true)
    (`MyCharacter.ExitADS` _playerref false)
    (`|PlayMontage` (`/Game/_GAME/Player/BP_Character.Mesh_1P` _playerref) "/Game/_GAME/ProceduralAnimation/Animations/FP_Montage_Reload.FP_Montage_Reload"
      (:`OnCompleted`
        (set `self.bReloading ?` false)))))

(event `self.Cancel Reload`
  (`AnimInstance.Montage_Stop` (`SkeletalMeshComponent.GetAnimInstance` (`/Game/_GAME/Player/BP_Character.Mesh_1P` (`self.PlayerRef`))) 0.0 "/Game/_GAME/ProceduralAnimation/Animations/FP_Montage_Reload.FP_Montage_Reload")
  (`SkeletalMeshComponent.Stop` (`self.GunMesh`)))

(event `self.Fire`
  (bind _recoilmaxthreshold_bp (`self.RecoilMaxThreshold BP`))
  (bind _returnvalue (`KismetMathLibrary.Abs` (.pitch (`KismetMathLibrary.NormalizedDeltaRotator` (`self.Origin Rotation BP`) (`self.Post Recoil Rotation BP`)))))
  (`parent.Fire` :!label _label_2)
  (`TimelineComponent.SetPlayRate` (`self.Recoil_TL`) 1.0)
  (`|ExecutionSequence`
    (:`then_0`
      (`/Engine/EditorBlueprintResources/StandardMacros.DoOnce` false :!label _label_3
        (:`Completed`
          (set `self.Origin Rotation BP` (`Controller.GetControlRotation` (`GameplayStatics.GetPlayerController` 0))))))
    (:`then_1`
      (bind (_direction _pitch_alpha _yaw_alpha) (`Timeline|Recoil_TL` :!label _label_4)
        (:`Update`
          (switch `ETimelineDirection` _direction
            (:`Forward`
              (`self.UpdatePlayerYawAndPitch` _pitch_alpha _yaw_alpha))
            (:`Backward`
              (`|ExecutionSequence`
                (:`then_0`
                  (`/Engine/EditorBlueprintResources/StandardMacros.DoOnce` false :!label _label_5
                    (:`Completed`
                      (set `self.Post Recoil Rotation BP` (`Controller.GetControlRotation` (`GameplayStatics.GetPlayerController` 0))))))
                (:`then_1`
                  (`self.UpdatePlayerYawAndPitch` (* _pitch_alpha -1.0 (select `bool` (> _returnvalue _recoilmaxthreshold_bp) :`false` (`KismetMathLibrary.MapRangeClamped` _returnvalue 0.0 _recoilmaxthreshold_bp 0.0 1.0) :`true` (`KismetMathLibrary.MapRangeClamped` _returnvalue (`self.RecoilMaxThreshold BP`) 30.0 1.0))) (* _yaw_alpha 0.0 0.0)))))))
        (:`Finished`
          (switch `ETimelineDirection` _direction
            (:`Backward`
              (`self.Reset_Recoil BP`))))))))

(event `Fire Start`
  (goto _label_2))

(event `self.Stop Fire`
  (`parent.Stop Fire` :!label _label_6)
  (`TimelineComponent.SetPlayRate` (`self.Recoil_TL`) 1.0)
  (goto _label_4 :!via `Reverse`))

(event `Reset_Recoil BP`
  (`|ExecutionSequence`
    (:`then_0`
      (goto _label_3 :!via `Reset`))
    (:`then_1`
      (goto _label_5 :!via `Reset`))))

(event `Fire Stop`
  (goto _label_6))

(fn `UpdatePlayerYawAndPitch`
  (params (Pitch :type "Float (double-precision)") (Yaw :type "Float (double-precision)"))
  (bind _returnvalue (`GameplayStatics.GetPlayerController` 0))
  (`PlayerController.AddPitchInput` _returnvalue (/ Pitch 7.0))
  (`PlayerController.AddYawInput` _returnvalue Yaw))

(fn `UserConstructionScript`
  (`parent.UserConstructionScript`))