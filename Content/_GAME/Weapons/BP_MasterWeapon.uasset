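; BP_MasterWeapon is a weapon pickup actor that, by its name, serves as the base for weapons.
; Sphere overlap by BP_Character shows or removes a WBP_Interact widget created with the weapon name; InteractPressed passes the weapon to the interactor's BP_WeaponSystemComponent.
; DeleteClass moves the actor above its gun mesh instead of destroying it.
; A camera line trace check compares the hit actor, with debug drawing and prints.
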(event `self.ReceiveTick`
  (params (DeltaSeconds :type "Float (single-precision)")))

(event `self.ReceiveBeginPlay`
  (bind _asbp_character (cast `/Game/_GAME/Player/BP_Character` (`GameplayStatics.GetPlayerCharacter` 0)))
  (bind _output_get (set `self.As BP Character` _asbp_character))
  (bind _returnvalue (`|CreateWidget` "/Game/_GAME/Widget/WBP_Interact.WBP_Interact_C" null (`self.WeaponName`)))
  (set `self.InteractiveWidget` _returnvalue)
  (`SceneComponent.SetHiddenInGame` (`self.InteractionIndicatorWidgetComp`) true false))

(event `ActorInterface.InteractPressed`
  (params (Interact_Actor :type "Actor Object Reference"))
  (`WeaponSystemComponent.PickUpWeapon` (`self.GetComponentByClass` Interact_Actor "/Game/_GAME/Weapons/BP_WeaponSystemCOmponent.BP_WeaponSystemComponent_C") self))

(event `ActorInterface.DeleteClass`
  (`self.K2_SetActorLocation` self (+ (`SceneComponent.K2_GetComponentLocation` (`self.GunMesh`)) (0.0 0.0 150.0)) false false))

(event `self.SphereComponent.OnComponentBeginOverlap`
  (params (OverlappedComponent :type "PrimitiveComponent Object Reference") (OtherActor :type "Actor Object Reference") (OtherComp :type "PrimitiveComponent Object Reference") (OtherBodyIndex :type Integer) (bFromSweep :type Boolean) (SweepResult :type "HitResult Structure (by ref)"))
  (cast `/Game/_GAME/Player/BP_Character` OtherActor)
  (`UserWidget.AddToViewport` (`self.InteractiveWidget`) 0))

(event `self.SphereComponent.OnComponentEndOverlap`
  (params (OverlappedComponent :type "PrimitiveComponent Object Reference") (OtherActor :type "Actor Object Reference") (OtherComp :type "PrimitiveComponent Object Reference") (OtherBodyIndex :type Integer))
  (cast `/Game/_GAME/Player/BP_Character` OtherActor)
  (`Widget.RemoveFromParent` (`self.InteractiveWidget`)))

(fn `BeginLineTraceToDeductWeapon`
  (returns (ReturnValue :type Boolean))
  (`parent.BeginLineTraceToDeductWeapon`)
  (`KismetSystemLibrary.PrintString` "Hello")
  (bind _returnvalue (`GameplayStatics.GetActorOfClass` "/Game/_GAME/Player/BP_Character.BP_Character_C"))
  (bind _camera (`/Game/_GAME/Player/BP_Character.Camera` _returnvalue))
  (bind _returnvalue_2 (`SceneComponent.K2_GetComponentLocation` _camera))
  (bind _outhit (`KismetSystemLibrary.LineTraceSingle` :`Start` _returnvalue_2 :`End` (+ _returnvalue_2 (* (`SceneComponent.GetForwardVector` _camera) 1000.0)) :`TraceChannel` "TraceTypeQuery1" :`DrawDebugType` "Persistent"))
  (bind (_bblockinghit _binitialoverlap _time _distance _location _impactpoint _normal _impactnormal _physmat _hitactor) (`GameplayStatics.BreakHitResult` _outhit))
  (`KismetSystemLibrary.PrintString` (`KismetSystemLibrary.GetDisplayName` _hitactor))
  (return (== null _hitactor)))

(fn `UserConstructionScript`)