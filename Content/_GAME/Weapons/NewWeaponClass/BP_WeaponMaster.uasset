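; Base weapon actor for guns that can be picked up, carried in hand or stowed in inventory, with state switching physics, collision and visibility.
; Sphere overlap shows an interact widget, and interacting hands the weapon to the character's BP_WeaponSystemComponent.
; FireHitScan traces from the muzzle along a random camera-forward cone, tightened by ADS and scaled by a recoil timeline, without processing the hit.
; Construction applies mesh and material; reload simply refills the clip.
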(event `Reload`
  (set `self.AmmoInClip` (`self.MaxAmmoInClip`)))

(event `Stow`)

(event `self.ReceiveBeginPlay`
  ;[1 1 1] Get Player Ref
  (bind _asbp_character (cast `/Game/_GAME/Player/BP_Character` (`GameplayStatics.GetPlayerCharacter` 0)))
  (set `self.PlayerRef` _asbp_character)
  (bind _returnvalue (`|CreateWidget` "/Game/_GAME/Widget/WBP_Interact.WBP_Interact_C" null (`self.WeaponName`)))
  (set `self.InteractiveWidget` _returnvalue)
  (`self.UpdateWeaponState` "EIR_OnGround"))

(event `Cancel Reload`)

(event `Equip`
  (set `MyCharacter.ADS_Offset` (`self.ADS_Offset_BP`) (`self.PlayerRef`)))

(event `ActorInterface.DeleteClass`
  (`self.K2_DestroyActor`))

(event `self.UpdateWeaponState`
  (params (WeaponState :type "EWeaponState Enum" :default "EIR_OnGround"))
  ;[0.5406 1 0.7476] Update weapon  state
  (switch `EWeaponState` WeaponState
    (:`EIR_OnGround`
      (`self.SetActorEnableCollision` true)
      (`PrimitiveComponent.SetSimulatePhysics` (`self.GunMesh`) true)
      (`self.SetActorHiddenInGame` false))
    (:`EIR_InHand`
      (`self.SetActorEnableCollision` false)
      (`PrimitiveComponent.SetSimulatePhysics` (`self.GunMesh`) false)
      (`self.SetActorHiddenInGame` false))
    (:`EIR_InInventory`
      (`self.SetActorEnableCollision` false)
      (`PrimitiveComponent.SetSimulatePhysics` (`self.GunMesh`) false)
      (`self.SetActorHiddenInGame` true))))

(event `self.SphereComponent.OnComponentBeginOverlap`
  (params (OverlappedComponent :type "PrimitiveComponent Object Reference") (OtherActor :type "Actor Object Reference") (OtherComp :type "PrimitiveComponent Object Reference") (OtherBodyIndex :type Integer) (bFromSweep :type Boolean) (SweepResult :type "HitResult Structure (by ref)"))
  ;[0.07239 0.4598 1] Pick Up widget
  (cast `/Game/_GAME/Player/BP_Character` OtherActor)
  (bind _returnvalue (`|CreateWidget` "/Game/_GAME/Widget/WBP_Interact.WBP_Interact_C" null (`self.WeaponName`)))
  (bind _output_get (set `self.InteractiveWidget` _returnvalue))
  (`UserWidget.AddToViewport` _output_get 0))

(event `self.SphereComponent.OnComponentEndOverlap`
  (params (OverlappedComponent :type "PrimitiveComponent Object Reference") (OtherActor :type "Actor Object Reference") (OtherComp :type "PrimitiveComponent Object Reference") (OtherBodyIndex :type Integer))
  ;[0.07239 0.4598 1] Pick Up widget
  (cast `/Game/_GAME/Player/BP_Character` OtherActor)
  (`Widget.RemoveFromParent` (stale `self.SphereComponent.OnComponentBeginOverlap` _output_get)))

(event `ActorInterface.InteractPressed`
  (params (Interact_Actor :type "Actor Object Reference"))
  ;[0.9929 1 0.487] Interact pressed Interface
  (`WeaponSystemComponent.PickUpWeapon` (`self.GetComponentByClass` Interact_Actor "/Game/_GAME/Weapons/BP_WeaponSystemCOmponent.BP_WeaponSystemComponent_C") self))

(event `Fire`
  (bind (_direction _recoil_alpha) (`Timeline|Recoil Alpha` :!via `PlayFromStart` :!label _label)
    (:`Update`
      (set `self.RecoilAlpha` _recoil_alpha))))

(event `Stop Fire`
  (goto _label :!via `Stop`))

(fn `Fire_HitScan`
  (params (`Draw debug` :type Boolean) (Spread :type "Float (double-precision)"))
  (bind _returnvalue (`SceneComponent.GetSocketLocation` (`self.GunMesh`) "Muzzle"))
  (`KismetSystemLibrary.LineTraceSingle` :`Start` _returnvalue :`End` (+ _returnvalue (* (`KismetMathLibrary.RandomUnitVectorInConeInDegrees` (`SceneComponent.GetForwardVector` (`/Game/_GAME/Player/BP_Character.Camera` (`self.PlayerRef`))) (* (/ Spread (`KismetMathLibrary.MapRangeClamped` (`MyCharacter.ADSAlpha` (`self.PlayerRef`)) 0.0 1.0 1.0 1.5)) (`self.RecoilAlpha`))) 20000.0)) :`TraceChannel` "TraceTypeQuery1" :`DrawDebugType` (select `bool` (`local.Draw debug`) :`true` "ForDuration" :!type "EDrawDebugTrace Enum"))
  (`self.Fire`))

(fn `UserConstructionScript`
  (`SkinnedMeshComponent.SetSkinnedAssetAndUpdate` (`self.GunMesh`) (`self.Mesh`) true)
  (`PrimitiveComponent.SetMaterial` (`self.GunMesh`) 0 (`self.Material`)))