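; Rifle weapon Blueprint that handles reload cancelling and holds a disconnected prototype of camera recoil with recovery.
; CancelReload stops the first-person reload montage on the player's arms and halts the gun mesh animation.
; The unwired recoil graph uses a timeline for random pitch/yaw kick, then scales pitch recovery by the deviation between saved control rotations.
; Reset_RecoilBP resets the DoOnce gates guarding those rotation snapshots.
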(event `self.Cancel Reload`
  (`AnimInstance.Montage_Stop` (`SkeletalMeshComponent.GetAnimInstance` (`/Game/_GAME/Player/BP_Character.Mesh_1P` (`self.PlayerRef`))) 0.0 "/Game/_GAME/ProceduralAnimation/Animations/FP_Montage_Reload.FP_Montage_Reload")
  (`SkeletalMeshComponent.Stop` (`self.GunMesh`)))

(event `Reset_Recoil BP`
  (`|ExecutionSequence`
    (:`then_0`
      (`/Engine/EditorBlueprintResources/StandardMacros.DoOnce` false :!via `Reset`
        (:`Completed`
          (set `self.Origin Rotation BP` (`Controller.GetControlRotation` (`GameplayStatics.GetPlayerController` 0))))))
    (:`then_1`
      (`/Engine/EditorBlueprintResources/StandardMacros.DoOnce` false :!via `Reset`
        (:`Completed`
          (set `self.Post Recoil Rotation BP` (`Controller.GetControlRotation` (`GameplayStatics.GetPlayerController` 0))))))))

(fn `UpdatePlayerYawAndPitch_0`
  (params (Pitch :type "Float (double-precision)") (Yaw :type "Float (double-precision)"))
  (bind _returnvalue (`GameplayStatics.GetPlayerController` 0))
  (`PlayerController.AddPitchInput` _returnvalue (/ Pitch 25.0))
  (`PlayerController.AddYawInput` _returnvalue (/ Yaw 50.0)))

(fn `UserConstructionScript`
  (`parent.UserConstructionScript`))