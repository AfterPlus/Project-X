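; BP_FN_EGLM is the FN EGLM grenade launcher weapon, built as a child Blueprint of a parent weapon class.
; On BeginPlay it calls the parent, then fills the WeaponDetails struct with its name, ammo capacity, fire rate and GunMesh skeletal mesh.
; WeaponFire is a stub that only prints a debug string, with no projectile or firing logic in this graph.
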(event `self.ReceiveBeginPlay`
  (`parent.ReceiveBeginPlay`)
  (setmembers `Weapon` :`StructRef` (`self.WeaponDetails`) :`WeaponName` "FN EGLM" :`MaxAmmo` 5 :`CurrentAmmo` 0 :`FireRate` 1.0 :`SkeletalMesh` (`self.GunMesh`) :`EquipWeapon` null :`WeaponReload` null))

(event `self.WeaponFire`
  (`KismetSystemLibrary.PrintString` "FN EGLM Fire"))

(fn `UserConstructionScript`
  (`parent.UserConstructionScript`))