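; BP_M4A1S is the M4A1S assault rifle weapon Blueprint, built on a parent weapon class.
; On BeginPlay it runs the parent logic, then fills its WeaponDetails struct with the name, ammo capacity, fire rate and gun mesh.
; WeaponFire currently only prints a debug message, with no firing logic in this Blueprint.
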(event `self.ReceiveBeginPlay`
  (`parent.ReceiveBeginPlay`)
  (setmembers `Weapon` :`StructRef` (`self.WeaponDetails`) :`WeaponName` "M4A1S" :`MaxAmmo` 30 :`CurrentAmmo` 0 :`FireRate` 1.0 :`SkeletalMesh` (`self.GunMesh`) :`EquipWeapon` null :`WeaponReload` null))

(event `self.WeaponFire`
  (`KismetSystemLibrary.PrintString` "M4 Fire" true true (struct :`R` 1.0 :`G` 0.675979 :`A` 1.0)))

(fn `UserConstructionScript`
  (`parent.UserConstructionScript`))