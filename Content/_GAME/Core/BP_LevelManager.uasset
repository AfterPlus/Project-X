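; BP_LevelManager is a level manager that pre-spawns enemies and triggers level expansion when an enemy is defeated.
; On BeginPlay it fills a SpawnedEnemies pool with BP_MasterEnemy actors at its own location.
; DeployEnemies moves the pool's first entry to a requested location without removing it from the array.
; EnemyDefeated has every spawned door in the current room try placing a random alley; remaining-enemy counting is left unconnected.
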(event `self.ReceiveBeginPlay`
  (`self.SpawnEnemies`))

(event `self.EnemyDefeated`
  (for _array_element (`Room.SpawnedDoors` (`MainGameModeBase.CurrentRoom` (`MainGameModeBase.GetInstance`)))
    (`Door.TryPlaceRandomAlley` _array_element)))

(event `self.SpawnEnemies`
  (for _ (range 51)
    (bind _returnvalue (`|SpawnActorFromClass` "/Game/_GAME/Enemies/BP_MasterEnemy.BP_MasterEnemy_C" (`KismetMathLibrary.MakeTransform` (`self.K2_GetActorLocation`)) "Undefined" "MultiplyWithRoot" null null))
    (`KismetArrayLibrary.Array_Add` (`self.SpawnedEnemies`) _returnvalue)))

(event `self.DeployEnemies`
  (params (SpawnLocation :type "Vector Structure"))
  (`self.K2_SetActorLocation` (`|GetArrayItem` (`self.SpawnedEnemies`)) SpawnLocation false false))

(fn `UserConstructionScript`)