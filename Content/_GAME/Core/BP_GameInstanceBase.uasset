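; BP_GameInstanceBase is the game instance that caches skill upgrade data and filters it by skill type.
; On Init, LoadSkills copies DT_Upgrades rows into the CachedSkill map, keyed by stringified row index.
; UpgradeSkillType clears SkillUpgrade and refills it with cached entries matching the requested type, also appending them to CachedSkillUpgrade, which is not cleared there.
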(event `self.LoadSkills`
  (bind _outrownames (`DataTableFunctionLibrary.GetDataTableRowNames` "/Game/_GAME/Data/DT_Upgrades.DT_Upgrades"))
  (for (_array_element _array_index) _outrownames
    (bind _returnvalue (`|GetDataTableRow` "/Game/_GAME/Data/DT_Upgrades.DT_Upgrades" _array_element)
      (:`then`
        (`BlueprintMapLibrary.Map_Add` (`self.CachedSkill`) (`KismetStringLibrary.Conv_IntToString` _array_index) _returnvalue)))))

(event `self.ReceiveInit`
  (`self.LoadSkills`))

(event `self.UpgradeSkillType`
  (params (SkillType :type "ESkillType Enum" :default "ESkillType_None"))
  (bind _cachedskill (`self.CachedSkill`))
  (`KismetArrayLibrary.Array_Clear` (`self.SkillUpgrade`))
  (bind _keys (`BlueprintMapLibrary.Map_Keys` _cachedskill))
  (for _array_element _keys
    (bind _value (`BlueprintMapLibrary.Map_Find` _cachedskill _array_element))
    (if (`|EnumEquality` (`.SkillType` (break `Upgrades` _value)) SkillType)
      (`KismetArrayLibrary.Array_Add` (`self.SkillUpgrade`) _value)
      (`KismetArrayLibrary.Array_Add` (`self.CachedSkillUpgrade`) _value))))