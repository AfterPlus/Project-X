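; Main game mode that acts as the level generator, pre-spawning the game's room and alley actors when play begins.
; BeginPlay calls the parent and Init, then spawns one actor per class in the Rooms and Alleys arrays.
; All spawn at a fixed point below the origin, with rooms rotated, and are stored in SpawnedRooms and SpawnedAlley.
; Each alley receives this game mode as its LevelGenerator reference.
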(event `Spawn Room`
  (for _array_element (`self.Rooms`)
    (bind _returnvalue (`|SpawnActorFromClass` _array_element (`KismetMathLibrary.MakeTransform` (0.0 0.0 -1000.0) (struct :`Yaw` 90.0)) "Undefined" "MultiplyWithRoot" null null))
    (`KismetArrayLibrary.Array_Add` (`self.SpawnedRooms`) _returnvalue)))

(event `Spawn Alley`
  (for _array_element (`self.Alleys`)
    (bind _returnvalue (`|SpawnActorFromClass` _array_element (`KismetMathLibrary.MakeTransform` (0.0 0.0 -1000.0)) "Undefined" "MultiplyWithRoot" null self null))
    (`KismetArrayLibrary.Array_Add` (`self.SpawnedAlley`) _returnvalue)))

(event `self.ReceiveBeginPlay`
  (`parent.ReceiveBeginPlay`)
  (`self.Init`)
  (`self.Spawn Room`)
  (`self.Spawn Alley`))

(fn `UserConstructionScript`)