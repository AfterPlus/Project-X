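; BP_PatrolRoute is an enemy patrol route that stores its waypoints as points on a spline.
; IncreamentPatrolRoute steps PatrolIndex by Direction, flipping Direction at the last and first points so the route ping-pongs instead of looping.
; GetSplinePointAsWorldPosition returns the world location of the spline point at the current PatrolIndex.
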(event `Increament Patrol Route`
  (bind _output_get (set `self.Patrol Index` (+ (`self.Patrol Index`) (`self.Direction`))))
  (if (== _output_get (- (`SplineComponent.GetNumberOfSplinePoints` (`self.Spline`)) 1))
    (set `self.Direction` -1)
    (elif (== (`self.Patrol Index`) 0)
      (set `self.Direction` 1))))

(fn `Get Spline point as world position`
  (returns (`Location ` :type "Vector Structure"))
  (return (`SplineComponent.GetLocationAtSplinePoint` (`self.Spline`) (`self.Patrol Index`) "World")))

(fn `UserConstructionScript`)