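; Gunner enemy run by a behavior tree that fires bullets and, at low health, can throw a grenade as a special attack.
; Shots reuse a random bullet from a small pool spawned out of view at BeginPlay.
; Custom primitive data drives spawn dissolve and hit flash; death ragdolls with an impulse at the hit bone, then dissolves and destroys the actor.
; A global grapple event pauses the AI for a fixed delay.
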(event `self.ReceiveBeginPlay`
  (`parent.ReceiveBeginPlay`)
  (`PrimitiveComponent.SetCustomPrimitiveDataFloat` (`self.Mesh`) 0 -100.0)
  (`PrimitiveComponent.SetCustomPrimitiveDataFloat` (`self.Mesh`) 1 0.0)
  (`|ExecutionSequence`
    (:`then_0`
      (bind (_direction _alpha) (`Timeline|Dissolve Material` :!via `PlayFromStart`)
        (:`Update`
          (`PrimitiveComponent.SetCustomPrimitiveDataFloat` (`self.Mesh`) 0 _alpha))
        (:`Finished`
          (set `self.bIsSpawned` true))))
    (:`then_1`
      (for _ (range 4)
        (bind _returnvalue (`|SpawnActorFromClass` "/Game/_GAME/Grenades/BP_EnemyBullet.BP_EnemyBullet_C" (`KismetMathLibrary.MakeTransform` (0.0 0.0 100000.0)) "Undefined" "MultiplyWithRoot" null null))
        (`KismetArrayLibrary.Array_Add` (`self.Bullets`) _returnvalue)))
    (:`then_2`
      (add `EventsHolder.Grapple` (`MainGameModeBase.EventsHolder` (`MainGameModeBase.GetInstance`)) (delegate `Grapple_Event`)))))

(event `Grapple_Event`
  (params (bUpdateTextOnly :type Boolean))
  (bind _returnvalue (`AIBlueprintHelperLibrary.GetAIController` (`self.GetController`)))
  (`BrainComponent.StopLogic` (`AIController.BrainComponent` _returnvalue) "")
  (`KismetSystemLibrary.Delay` 3.0) ; This delay should come from skill tree
  (`AIController.RunBehaviorTree` _returnvalue "/Game/_GAME/Enemies/BP_Gunner/AI/BT_Gunner.BT_Gunner"))

(event `ActorInterface.PlaySpecialAttack`
  (`|PlayMontage` (`self.Mesh`) "/Game/Mixamo/Throw_Montage.Throw_Montage" 1.0 0.0 "None"))

(event `Equip Grenade`
  (bind _grenade (`self.Grenade`))
  ;[1 1 1] Equip Grenade
  (`MasterGrenade.ResetProperties` _grenade)
  (`self.K2_AttachToComponent` _grenade (`self.Mesh`) "RightHand" "SnapToTarget" "SnapToTarget" "SnapToTarget" false)
  (`KismetSystemLibrary.Delay` 0.6)
  (`self.K2_DetachFromActor` (`self.Grenade`) "KeepWorld" "KeepWorld" "KeepWorld")
  (`MasterGrenade.EnemyThrow` (`self.Grenade`) (+ (* (`self.GetActorForwardVector`) 150.0) (* (`self.GetActorRightVector`) 320.0))))

(event `ActorInterface.EnemyFire`
  ;[1 1 1] Fire
  (bind _output_get (set `self.Current Spawn Bullet` (`KismetArrayLibrary.Array_Random` (`self.Bullets`))))
  (`self.K2_SetActorLocation` _output_get (`SceneComponent.GetSocketLocation` (`self.Mesh`) "BulletSpawn") false false)
  (`EnemyBullet.AddImpulse` (`self.Current Spawn Bullet`)))

(event `ActorInterface.CheckForEnemiesRange`
  (params (bIsInRange :type Boolean))
  (set `self.bIsInPlayersAttackRange` bIsInRange))

(event `ActorInterface.ApplyDamageToEnemy`
  (params (Damage :type "Float (single-precision)"))
  ;[1 1 1] Apply damage
  (if (< (- (`self.Health`) Damage) 1.0)
    (`self.Death`)
    (else
      (set `self.Health` (- (`self.Health`) Damage))))
  (if (not (`TimelineComponent.IsPlaying` (`self.Hit Effect`)))
    (`PrimitiveComponent.SetCustomPrimitiveDataFloat` (`self.Mesh`) 1 1.0)
    (`Timeline|Hit Effect` :!via `PlayFromStart`
      (:`Finished`
        (`PrimitiveComponent.SetCustomPrimitiveDataFloat` (`self.Mesh`) 1 0.0)))))

(event `Death`
  (bind _mesh (`self.Mesh`))
  (bind (_returnvalue_x _returnvalue_y) (`KismetMathLibrary.BreakVector` (* (* (`self.GetActorForwardVector` (`MyCharacter.GetInstance`)) 3000.0) 1.0)))
  ;[1 1 1] Death
  (`PrimitiveComponent.SetCollisionProfileName` (`self.CapsuleComponent`) "NoCollision" true)
  (`PrimitiveComponent.SetSimulatePhysics` _mesh true)
  (`PrimitiveComponent.AddImpulse` _mesh (`KismetMathLibrary.MakeVector` _returnvalue_x _returnvalue_y) (`KismetStringLibrary.Conv_StringToName` (`MasterWeapon.BoneHitName` (`MyCharacter.InHandWeapon` (`MyCharacter.GetInstance`)))) true)
  (`EventsHolder.EnemyDead` (`MainGameModeBase.EventsHolder` (`MainGameModeBase.GetInstance`)))
  (`BrainComponent.StopLogic` (`AIController.BrainComponent` (`AIBlueprintHelperLibrary.GetAIController` (`self.GetController`))) "")
  (`CharacterMovementComponent.SetMovementMode` (`self.CharacterMovement`) "MOVE_None" 0)
  (`KismetSystemLibrary.Delay` 2.0)
  (`TimelineComponent.Reverse` (`self.Dissolve Material `))
  (`KismetSystemLibrary.Delay` 3.0)
  (`self.K2_DestroyActor`))

(fn `CanPerformSpecialAttack`
  (returns (ReturnValue :type Boolean))
  (return (< (`self.Health`) 30.0)))

(fn `UserConstructionScript`
  (`parent.UserConstructionScript`))