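; BP_GunnerDummy is an enemy character, apparently a stand-in gunner, whose Attack event only prints a debug string.
; It exposes its patrol route through GetPatrolRoute.
; SetMovementSpeed maps a movement state from idle to sprinting onto the CharacterMovement max walk speed and returns the applied value.
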(event `Attack`
  (`KismetSystemLibrary.PrintString` "attack"))

(fn `GetPatrolRoute`
  (returns (Route :type "/Game/_GAME/Enemies/BP_PatrolRoute Object Reference"))
  (return (`self.Patrol Route`)))

(fn `Set MovementSpeed`
  (params (Speed :type "/Game/_GAME/Enemies/AI/Enum/E_MovementSpeed Enum" :default "NewEnumerator0"))
  (returns (`Speed Value` :type "Float (double-precision)"))
  (bind _output_get (set `CharacterMovementComponent.MaxWalkSpeed` (select `/Game/_GAME/Enemies/AI/Enum/E_MovementSpeed` Speed :`NewEnumerator1` 100.0 :`NewEnumerator2` 300.0 :`NewEnumerator3` 500.0 :!type "Float (single-precision)") (`self.CharacterMovement`)))
  (return _output_get))

(fn `UserConstructionScript`
  (`parent.UserConstructionScript`))