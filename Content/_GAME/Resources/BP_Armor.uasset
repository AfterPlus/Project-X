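; BP_Armor is an armor pickup that grants the player armor when picked up.
; On pickup it checks that the instance's armor is below 100, then calls UpdatePlayerArmor on the instance's EventsHolder with a fixed amount and itself as the source actor.
; The change is delegated to that event holder, and BeginPlay is left disabled.
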(event `self.On PickUp`
  (bind _returnvalue (`MyCharacter.GetInstance`))
  (if (< (`MyCharacter.Armor` _returnvalue) 100.0)
    (bind _returnvalue_2 (`MainGameModeBase.GetInstance`))
    (`EventsHolder.UpdatePlayerArmor` (`MainGameModeBase.EventsHolder` _returnvalue_2) 50.0 self)))

(fn `UserConstructionScript`
  (`parent.UserConstructionScript`))