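; BP_Nade_Decoy is a pickup actor for a decoy grenade.
; On pickup, it passes the decoy type to the BP_GrenadeSystemComponent found on the object returned by GetInstance.
; It then fires a pickup notification with its icon and name through that object's EventsHolder and destroys itself.
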(event `self.On PickUp`
  (bind _returnvalue (`MyCharacter.GetInstance`))
  (`GrenadeSystemComponent.PickUp` (`self.GetComponentByClass` _returnvalue "/Game/_GAME/Grenades/BP_GrenadeSystemComponent.BP_GrenadeSystemComponent_C") "EGrenadeType_Decoy")
  (bind _returnvalue_2 (`MainGameModeBase.GetInstance`))
  (`EventsHolder.PickUpNotification` (`MainGameModeBase.EventsHolder` _returnvalue_2) (`self.Icon`) "Decoy" "1")
  (`self.K2_DestroyActor`))

(fn `UserConstructionScript`
  (`parent.UserConstructionScript`))