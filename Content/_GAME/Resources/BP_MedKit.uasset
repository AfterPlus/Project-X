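; BP_MedKit is a health pickup that restores a fixed amount of player health when picked up.
; On pickup it acts only if the GetInstance health is below 100, broadcasting health update and pickup notification events through the EventsHolder, then destroys itself.
; The construction script sets the mesh to a fixed rotation.
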(event `self.On PickUp`
  (bind _returnvalue (`MyCharacter.GetInstance`))
  (if (< (`MyCharacter.Health` _returnvalue) 100.0)
    (bind _returnvalue_2 (`MainGameModeBase.GetInstance`))
    (`EventsHolder.UpdatePlayerHealth` (`MainGameModeBase.EventsHolder` _returnvalue_2) 25.0 self)
    (bind _returnvalue_3 (`MainGameModeBase.GetInstance`))
    (`EventsHolder.PickUpNotification` (`MainGameModeBase.EventsHolder` _returnvalue_3) (`self.Icon`) "Health" "25")
    (`self.K2_DestroyActor`)))

(fn `UserConstructionScript`
  (`parent.UserConstructionScript`)
  (`SceneComponent.K2_SetWorldRotation` (`self.Mesh`) (struct :`Roll` 90.0) false false))