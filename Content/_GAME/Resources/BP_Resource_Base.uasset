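; BP_Resource_Base is a resource pickup that gives a character 10 units of its resource type.
; On sphere overlap it casts to BP_Character and adds to that character's Resources map, keyed by the pickup's own class.
; DestroyActor runs before the cast, so any overlapping actor removes the pickup.
; A disconnected fragment references adding a child to the weapon wheel's grenade list.
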(event `self.ReceiveBeginPlay`)

(event `self.Sphere.OnComponentBeginOverlap`
  (params (OverlappedComponent :type "PrimitiveComponent Object Reference") (OtherActor :type "Actor Object Reference") (OtherComp :type "PrimitiveComponent Object Reference") (OtherBodyIndex :type Integer) (bFromSweep :type Boolean) (SweepResult :type "HitResult Structure (by ref)"))
  (bind _returnvalue (`GameplayStatics.GetObjectClass` self))
  (`self.K2_DestroyActor`)
  (bind _asbp_character (cast `/Game/_GAME/Player/BP_Character` OtherActor))
  (bind _resources (`/Game/_GAME/Player/BP_Character.Resources` _asbp_character))
  (`BlueprintMapLibrary.Map_Add` _resources _returnvalue (+ (`BlueprintMapLibrary.Map_Find` _resources _returnvalue) 10))
  (`self.K2_DestroyActor`))

(fn `UserConstructionScript`)