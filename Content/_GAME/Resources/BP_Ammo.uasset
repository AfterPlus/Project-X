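; BP_Ammo is an ammo actor that launches itself along a randomized arc when it spawns.
; On BeginPlay it sets the ProjectileMovement velocity from a negated, randomly scaled X of its Vector value, a random sideways Y and a random upward Z.
; An unconnected loop for picking random values at least a set distance apart is left in the graph and never runs.
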(event `self.ReceiveBeginPlay`
  (bind _returnvalue_x (`KismetMathLibrary.BreakVector` (* (`self.Vector`) (`KismetMathLibrary.RandomFloatInRange` 80.0 90.0))))
  (set `MovementComponent.Velocity` (`KismetMathLibrary.MakeVector` (* _returnvalue_x -1.0) (* (`KismetMathLibrary.RandomFloatInRange` -50.0 50.0) (`KismetMathLibrary.RandomFloatInRange` -5.0 5.0)) (`KismetMathLibrary.RandomFloatInRange` 150.0 200.0)) (`self.ProjectileMovement`)))

(fn `UserConstructionScript`)