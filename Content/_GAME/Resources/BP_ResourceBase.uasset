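; BP_ResourceBase is a base Blueprint for resource pickups collected by the player character.
; On BeginPlay it sets a randomised ProjectileMovementComponent velocity, tossing the resource upward with horizontal scatter.
; A Sphere overlap with BP_Character calls OnPickUp, an empty event that appears intended for child classes to override.
; The base itself applies no reward and does not destroy itself.
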(event `self.ReceiveBeginPlay`
  (bind _returnvalue_x (`KismetMathLibrary.BreakVector` (* (`self.Vector`) (`KismetMathLibrary.RandomFloatInRange` 80.0 90.0))))
  (set `MovementComponent.Velocity` (`KismetMathLibrary.MakeVector` (* _returnvalue_x -1.0) (* (`KismetMathLibrary.RandomFloatInRange` -50.0 50.0) (`KismetMathLibrary.RandomFloatInRange` -5.0 5.0)) (`KismetMathLibrary.RandomFloatInRange` 150.0 200.0)) (`self.ProjectileMovementComponent`)))

(event `On PickUp`)

(event `self.Sphere.OnComponentBeginOverlap`
  (params (OverlappedComponent :type "PrimitiveComponent Object Reference") (OtherActor :type "Actor Object Reference") (OtherComp :type "PrimitiveComponent Object Reference") (OtherBodyIndex :type Integer) (bFromSweep :type Boolean) (SweepResult :type "HitResult Structure (by ref)"))
  (cast `/Game/_GAME/Player/BP_Character` OtherActor)
  (`self.On PickUp`))

(fn `UserConstructionScript`)