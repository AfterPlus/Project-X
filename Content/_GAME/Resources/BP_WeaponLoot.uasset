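; BP_WeaponLoot is a world pickup that gives the interacting actor a weapon, currently hardcoded to BP_AK47.
; On BeginPlay it pre-spawns the weapon actor far below the origin and keeps a reference.
; Sphere overlaps with BP_Character show and remove a WBP_Interact prompt carrying the weapon's name.
; InteractPressed passes the stored weapon to the interactor's BP_WeaponSystemComponent, then destroys the loot actor.
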(event `self.ReceiveBeginPlay`
  (`parent.ReceiveBeginPlay`)
  (bind _returnvalue (`|SpawnActorFromClass` "/Game/_GAME/Weapons/WeaponClass/BP_AK-47.BP_AK-47_C" (`KismetMathLibrary.MakeTransform` (0.0 0.0 -10000.0)) "Undefined" "MultiplyWithRoot" null null))
  (set `self.Spawn Weapon` _returnvalue))

(event `ActorInterface.InteractPressed`
  (params (Interact_Actor :type "Actor Object Reference"))
  (`WeaponSystemComponent.PickUpWeapon` (`self.GetComponentByClass` Interact_Actor "/Game/_GAME/Weapons/BP_WeaponSystemCOmponent.BP_WeaponSystemComponent_C") (`self.Spawn Weapon`))
  (`self.K2_DestroyActor`))

(event `self.Sphere.OnComponentBeginOverlap`
  (params (OverlappedComponent :type "PrimitiveComponent Object Reference") (OtherActor :type "Actor Object Reference") (OtherComp :type "PrimitiveComponent Object Reference") (OtherBodyIndex :type Integer) (bFromSweep :type Boolean) (SweepResult :type "HitResult Structure (by ref)"))
  (cast `/Game/_GAME/Player/BP_Character` OtherActor)
  (bind _returnvalue (`|CreateWidget` "/Game/_GAME/Widget/WBP_Interact.WBP_Interact_C" null (`MasterWeapon.WeaponName` (`self.Spawn Weapon`))))
  (bind _output_get (set `self.InteractiveWidget` _returnvalue))
  (`UserWidget.AddToViewport` _output_get 0))

(event `self.Sphere.OnComponentEndOverlap`
  (params (OverlappedComponent :type "PrimitiveComponent Object Reference") (OtherActor :type "Actor Object Reference") (OtherComp :type "PrimitiveComponent Object Reference") (OtherBodyIndex :type Integer))
  (cast `/Game/_GAME/Player/BP_Character` OtherActor)
  (`Widget.RemoveFromParent` (stale `self.Sphere.OnComponentBeginOverlap` _output_get)))

(fn `UserConstructionScript`
  (`parent.UserConstructionScript`)
  (`SceneComponent.K2_SetWorldRotation` (`self.Mesh`) (struct :`Roll` 90.0) false false))