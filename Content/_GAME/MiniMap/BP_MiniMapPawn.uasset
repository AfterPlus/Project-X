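; BP_MiniMapPawn is a pawn used for the minimap view, letting the player look around until returning to the main character.
; It caches the player's BP_Character on BeginPlay and feeds Turn and LookUp axes into controller rotation.
; Pressing Space Bar makes the player controller possess that character again and removes the character's MiniMapTest widget from the screen.
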(event `self.ReceiveBeginPlay`
  (bind _asbp_character (cast `/Game/_GAME/Player/BP_Character` (`GameplayStatics.GetPlayerCharacter` 0)))
  (set `self.As BP Character` _asbp_character))

(event `Key|SpaceBar`
  (params (Key :type "Key Structure"))
  (bind _as_bp_character (`self.As BP Character`))
  (:`Pressed`
    (`Controller.Possess` (`GameplayStatics.GetPlayerController` 0) _as_bp_character)
    (`Widget.RemoveFromParent` (`/Game/_GAME/Player/BP_Character.MiniMapTest` _as_bp_character))))

(event `InputAxis|LookUp`
  (params (AxisValue :type "Float (single-precision)"))
  (`self.AddControllerPitchInput` AxisValue))

(event `InputAxis|Turn`
  (params (AxisValue :type "Float (single-precision)"))
  (`self.AddControllerYawInput` AxisValue))

(fn `UserConstructionScript`)