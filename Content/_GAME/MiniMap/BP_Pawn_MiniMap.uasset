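; BP_Pawn_MiniMap is a controllable minimap camera pawn with movement, right-mouse yaw rotation and clamped, lerped spring-arm zoom.
; On BeginPlay it caches the player BP_Character and adds registered markers to the scene capture's show-only list.
; Marker update events snap the pawn to the character's location.
; A thumb mouse button clears all widgets and repossesses the character; Tick only prints a debug string.
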(event `self.ReceiveTick`
  (params (DeltaSeconds :type "Float (single-precision)"))
  (`KismetSystemLibrary.PrintString` "Hello"))

(event `self.ReceiveBeginPlay`
  (bind _asbp_character (cast `/Game/_GAME/Player/BP_Character` (`GameplayStatics.GetPlayerCharacter` 0)))
  (set `self.As BP Character` _asbp_character)
  (bind _returnvalue (`MainGameModeBase.GetInstance`))
  (`/Engine/EditorBlueprintResources/StandardMacros.IsValid` _returnvalue
    (:`Is Valid`
      (add `EventsHolder.UpdateMiniMapMarkerReq` (`MainGameModeBase.EventsHolder` _returnvalue) (delegate `CustomEvent_0`))
      (bind _returnvalue_2 (`MiniMap.GetInstance`))
      (for _array_element (`MiniMap.MiniMapMarkers` _returnvalue_2)
        (`SceneCaptureComponent.ShowOnlyComponent` (`self.CaptureComponent2D`) _array_element)))))

(event `CustomEvent_0`
  (params (Actor :type "Actor Object Reference") (Location :type "Vector Structure") (Marker :type "EMarkerType Enum" :default "EMarkerType_None"))
  (`self.K2_SetActorLocation` (`self.K2_GetActorLocation` (`self.As BP Character`))))

(event `InputAxis|MoveForward`
  (params (AxisValue :type "Float (single-precision)"))
  (`self.K2_AddActorWorldOffset` (* (`self.GetActorForwardVector`) (* AxisValue (* (`self.MoveSpeed`) 1.0)))))

(event `Key|ThumbMouseButton2`
  (params (Key :type "Key Structure"))
  (:`Pressed`
    (`WidgetLayoutLibrary.RemoveAllWidgets`)
    (`Controller.Possess` (`GameplayStatics.GetPlayerController` 0) (`self.As BP Character`))))

(event `InputAxis|MoveRight`
  (params (AxisValue :type "Float (single-precision)"))
  (`self.K2_AddActorWorldOffset` (* (`self.GetActorRightVector`) (* AxisValue (* (`self.MoveSpeed`) 1.0)))))

(event `InputAxis|MiniMap Pan X`
  (params (AxisValue :type "Float (single-precision)"))
  (if (== AxisValue 0.0)
    _
    (elif (`PlayerController.IsInputKeyDown` (`GameplayStatics.GetPlayerController` 0) "RightMouseButton")
      (`self.K2_AddActorWorldRotation` (`KismetMathLibrary.MakeRotator` 0.0 0.0 (* AxisValue (`self.CameraRotationSpeed`)))))))

(event `InputAxis|Mini Map Zoom`
  (params (AxisValue :type "Float (single-precision)"))
  (if (not (== AxisValue 0.0))
    (set `SpringArmComponent.TargetArmLength` (`KismetMathLibrary.Lerp` (`SpringArmComponent.TargetArmLength` (`self.SpringArmComponent`)) (`KismetMathLibrary.FClamp` (+ (`SpringArmComponent.TargetArmLength` (`self.SpringArmComponent`)) (* AxisValue (* (`self.ZoomSpeed`) -1.0))) (`self.MinZoom`) (`self.MaxZoom`)) 0.5) (`self.SpringArmComponent`))))

(fn `UserConstructionScript`
  (`SceneComponent.K2_SetWorldRotation` (`self.SpringArmComponent`) (struct :`Pitch` 320.0) false false))