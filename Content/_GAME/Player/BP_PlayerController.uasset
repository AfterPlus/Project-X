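; Player controller Blueprint that handles opening the skill upgrade screen and a time-scale hotkey.
; ShowUpgradeWidget adds the skill upgrades widget held by the game instance to the viewport, switches to UI-only input and shows the cursor.
; Ctrl+mouse wheel toggles global time dilation between slow motion and normal speed.
; BeginPlay is empty, and the main menu creation logic is left disconnected, so it never runs.
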(event `self.ReceiveBeginPlay`)

(event `self.ShowUpgradeWidget`
  (bind _returnvalue (`GameplayStatics.GetPlayerController` 0))
  (`UserWidget.AddToViewport` (`MainHUD.Wbp_SkillUpgrades` (`MainHUD.GetInstance`)) 0)
  (`WidgetBlueprintLibrary.SetInputMode_UIOnlyEx` _returnvalue null "DoNotLock" true)
  (set `PlayerController.bShowMouseCursor` true _returnvalue))

(event `Key|Ctrl+MouseScrollUp`
  (params (Key :type "Key Structure"))
  (:`Pressed`
    (`GameplayStatics.SetGlobalTimeDilation` 1.0)))

(event `Key|Ctrl+MouseScrollDown`
  (params (Key :type "Key Structure"))
  (:`Pressed`
    (`GameplayStatics.SetGlobalTimeDilation` 0.1)))

(fn `UserConstructionScript`)