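; Anim notify that forwards a named event from an animation to the owning actor's AnimComp component.
; On firing, it finds AnimComp on the mesh owner and, if valid, calls its Notify with the configured NotifyName converted to a Name.
; The notify also displays NotifyName as its label in the animation editor.
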(fn `GetNotifyName`
  (returns (ReturnValue :type String))
  (return (`self.NotifyName`)))

(fn `Received_Notify`
  (params (MeshComp :type "SkeletalMeshComponent Object Reference") (Animation :type "AnimSequenceBase Object Reference"))
  (returns (ReturnValue :type Boolean))
  (locals (AnimComp :type "/Game/Defender/Blueprints/Components/AnimComp Object Reference"))
  (bind _output_get (set `local.AnimComp` (`Actor.GetComponentByClass` (`ActorComponent.GetOwner` MeshComp) "/Game/Defender/Blueprints/Components/AnimComp.AnimComp_C")))
  (`/Engine/EditorBlueprintResources/StandardMacros.IsValid` _output_get
    (:`Is Valid`
      (`/Game/Defender/Blueprints/Components/AnimComp.Notify` (`local.AnimComp`) (`KismetStringLibrary.Conv_StringToName` (`self.NotifyName`)))
      (return false))))