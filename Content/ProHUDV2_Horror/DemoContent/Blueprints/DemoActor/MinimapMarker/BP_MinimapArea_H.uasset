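; BP_MinimapArea_H is a demo trigger volume that toggles the HUD minimap as the player walks in and out of its box.
; On overlap by ThirdPersonCharacter_H, it asks the HUD manager to show and update the minimap.
; On exit, it hides the minimap, removes all markers, and calls UpdateMarker(false) on every BP_DemoTrigger_Marker in the level.
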(event `self.Box.OnComponentBeginOverlap`
  (params (OverlappedComponent :type "PrimitiveComponent Object Reference") (OtherActor :type "Actor Object Reference") (OtherComp :type "PrimitiveComponent Object Reference") (OtherBodyIndex :type Integer) (bFromSweep :type Boolean) (SweepResult :type "HitResult Structure (by ref)"))
  (bind _hud_manager (`/Game/ProHUDV2_Horror/Blueprints/Libraries/BP_PHV2_Functions_H.GetHUDManager_H`))
  (cast `/Game/ProHUDV2_Horror/DemoContent/DemoCharacter/ThirdPersonCharacter_H` OtherActor)
  (`/Game/ProHUDV2_Horror/Blueprints/Libraries/BPi_HUDManagerV2_H.ShowMinimap_H` _hud_manager 0)
  (`/Game/ProHUDV2_Horror/Blueprints/Libraries/BPi_HUDManagerV2_H.UpdateMinimap_H` _hud_manager 1.0))

(event `self.Box.OnComponentEndOverlap`
  (params (OverlappedComponent :type "PrimitiveComponent Object Reference") (OtherActor :type "Actor Object Reference") (OtherComp :type "PrimitiveComponent Object Reference") (OtherBodyIndex :type Integer))
  (bind _hud_manager (`/Game/ProHUDV2_Horror/Blueprints/Libraries/BP_PHV2_Functions_H.GetHUDManager_H`))
  (cast `/Game/ProHUDV2_Horror/DemoContent/DemoCharacter/ThirdPersonCharacter_H` OtherActor)
  (`/Game/ProHUDV2_Horror/Blueprints/Libraries/BPi_HUDManagerV2_H.HideMinimap_H` _hud_manager)
  (`/Game/ProHUDV2_Horror/Blueprints/Libraries/BPi_HUDManagerV2_H.RemoveAllMinimapMarkers_H` _hud_manager)
  (bind _outactors (`GameplayStatics.GetAllActorsOfClass` "/Game/ProHUDV2_Horror/DemoContent/DemoRoom/DemoTrigger/BP_DemoTrigger_Marker.BP_DemoTrigger_Marker_C"))
  (for _array_element _outactors
    (`/Engine/EditorBlueprintResources/StandardMacros.IsValid` _array_element
      (:`Is Valid`
        (`/Game/ProHUDV2_Horror/DemoContent/DemoRoom/DemoTrigger/BP_DemoTrigger_Marker.UpdateMarker` _array_element false)))))

(fn `UserConstructionScript`)